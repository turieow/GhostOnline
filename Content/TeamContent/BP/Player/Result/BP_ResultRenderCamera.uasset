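; Result-screen actor that renders one player's character into that player's render target through a SceneCapture limited to showing itself.
; It dresses the mesh as the ghost bear or a colored human from the current game number, then picks montage and win/sad Niagara effect from game state or final rank (Juni).
; On final results the first-place crown spins, lowers by timeline onto CrownSocket, attaches, and releases the anim wait.
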(event `self.ReceiveBeginPlay`
  (bind _isfinalresult (`self.IsFinalResult`))
  (`KismetArrayLibrary.Array_Add` (`SceneCaptureComponent.ShowOnlyActors` (`self.SceneCaptureComponent2D`)) self)
  (`self.E_SetTextureTarget`)
  (`self.E_SetModel`)
  (message `/Game/TeamContent/BP/Player/Result/BPI_ResultCharacterInterface.InitResultAnimation` (`SkeletalMeshComponent.GetAnimInstance` (`self.MainMesh`)) (`self.Juni`) _isfinalresult)
  (message `/Game/TeamContent/BP/Player/Result/BPI_ResultCharacterInterface.InitResultAnimation` (`SkeletalMeshComponent.GetAnimInstance` (`self.GhostMesh`)) (`self.Juni`) _isfinalresult)
  (if (`self.IsFinalResult`)
    (`SceneComponent.SetVisibility` (`self.SM_CrownMesh`) (`self.GetCrownVisibility`) false)
    (`self.E_CrownMeshMove`)))

(event `E_SetTextureTarget`
  ;[1 1 1] テクスチャターゲット設定
  (set `SceneCaptureComponent2D.TextureTarget` (select `int` (`self.PlayerInde`) :`0` "/Game/TeamContent/Graphic/Material/UI/ResultUI/RT_Player0.RT_Player0" :`1` "/Game/TeamContent/Graphic/Material/UI/ResultUI/RT_Player1.RT_Player1" :`2` "/Game/TeamContent/Graphic/Material/UI/ResultUI/RT_Player2.RT_Player2" :`3` "/Game/TeamContent/Graphic/Material/UI/ResultUI/RT_Player3.RT_Player3" :!type "TextureRenderTarget2D Object Reference") (`self.SceneCaptureComponent2D`)))

(event `E_SetModel`
  ;[1 1 1] 見た目変更
  (bind _currentgamenum (message `/Game/TeamContent/BP/System/GameInstance/BPI_GameInstanceInterface.GetCurrentGameNum` (`GameplayStatics.GetGameInstance`)))
  (if (== _currentgamenum (`self.PlayerInde`))
    (`self.E_GhostSetUp`)
    (else
      (`self.E_HumanSetUp`))))

(event `E_GhostSetUp`
  ;[1 1 1] お化け用セットアップ
  (`SkinnedMeshComponent.SetSkinnedAssetAndUpdate` (`self.MainMesh`) "/Game/TeamContent/Graphic/Mesh/Character/SK_Bear.SK_Bear" true)
  (`PrimitiveComponent.SetMaterial` (`self.MainMesh`) 0 "/Game/TeamContent/Graphic/Material/Chara/MI_Chara/MI_BaseTranse1.MI_BaseTranse1")
  (`PrimitiveComponent.SetMaterial` (`self.MainMesh`) 1 "/Game/TeamContent/Graphic/Material/Chara/MI_Chara/MI_BaseTranse1.MI_BaseTranse1")
  (`SkeletalMeshComponent.SetAnimInstanceClass` (`self.MainMesh`) "/Game/TeamContent/Graphic/Animation/Result/ABP_ResultBear.ABP_ResultBear_C")
  (bind _state (message `/Game/TeamContent/BP/System/MainGame/BPI_GameModeInterface.GetGameState` (`GameplayStatics.GetGameMode`)))
  (`AnimInstance.Montage_Play` (`SkeletalMeshComponent.GetAnimInstance` (`self.MainMesh`)) (select `/Game/TeamContent/BP/Enum/En_GameState` _state :!type "AnimMontage Object Reference") 1.0 "MontageLength" 0.0 true)
  (if (`self.IsFinalResult`)
    (`NiagaraComponent.SetAsset` (`self.Niagara`) (select `bool` (== (`self.Juni`) 0) :`false` "/Game/TeamContent/Graphic/Particle/NPS_Sad.NPS_Sad" :`true` "/Game/TeamContent/Graphic/Particle/NPS_Win.NPS_Win" :!type "NiagaraSystem Object Reference") true)
    (else
      (`NiagaraComponent.SetAsset` (`self.Niagara`) (select `/Game/TeamContent/BP/Enum/En_GameState` _state :`NewEnumerator1` "/Game/TeamContent/Graphic/Particle/NPS_Win.NPS_Win" :`NewEnumerator2` "/Game/TeamContent/Graphic/Particle/NPS_Sad.NPS_Sad" :`NewEnumerator3` "/Game/TeamContent/Graphic/Particle/NPS_Sad.NPS_Sad" :!type "NiagaraSystem Object Reference") true))))

(event `E_HumanSetUp`
  (bind _mainmesh (`self.MainMesh`))
  ;[1 1 1] 人間用セットアップ
  (`SkinnedMeshComponent.SetSkinnedAssetAndUpdate` _mainmesh "/Game/TeamContent/Graphic/Mesh/Character/SK_Human.SK_Human" true)
  (for _index (range (`PrimitiveComponent.GetNumMaterials` _mainmesh))
    (`PrimitiveComponent.SetMaterial` (`self.MainMesh`) _index (select `int` (`self.PlayerInde`) :`0` "/Game/TeamContent/Graphic/Material/Chara/MI_Chara/MI_Human_1P.MI_Human_1P" :`1` "/Game/TeamContent/Graphic/Material/Chara/MI_Chara/MI_Human_2P.MI_Human_2P" :`2` "/Game/TeamContent/Graphic/Material/Chara/MI_Chara/MI_Human_3P.MI_Human_3P" :`3` "/Game/TeamContent/Graphic/Material/Chara/MI_Chara/MI_Human_4P.MI_Human_4P" :!type "MaterialInterface Object Reference")))
  (`SceneComponent.SetVisibility` (`self.GhostMesh`) false false)
  (bind _state (message `/Game/TeamContent/BP/System/MainGame/BPI_GameModeInterface.GetGameState` (`GameplayStatics.GetGameMode`)))
  (`AnimInstance.Montage_Play` (`SkeletalMeshComponent.GetAnimInstance` (`self.MainMesh`)) (select `/Game/TeamContent/BP/Enum/En_GameState` _state :!type "AnimMontage Object Reference") 1.0 "MontageLength" 0.0 true)
  (if (`self.IsFinalResult`)
    (`NiagaraComponent.SetAsset` (`self.Niagara`) (select `bool` (== (`self.Juni`) 0) :`false` "/Game/TeamContent/Graphic/Particle/NPS_Sad.NPS_Sad" :`true` "/Game/TeamContent/Graphic/Particle/NPS_Win.NPS_Win" :!type "NiagaraSystem Object Reference") true)
    (else
      (`NiagaraComponent.SetAsset` (`self.Niagara`) (select `/Game/TeamContent/BP/Enum/En_GameState` _state :`NewEnumerator1` "/Game/TeamContent/Graphic/Particle/NPS_Sad.NPS_Sad" :`NewEnumerator2` "/Game/TeamContent/Graphic/Particle/NPS_Win.NPS_Win" :`NewEnumerator3` "/Game/TeamContent/Graphic/Particle/NPS_Sad.NPS_Sad" :!type "NiagaraSystem Object Reference") true))))

(event `self.ReceiveTick`
  (params (DeltaSeconds :type "Float (single-precision)"))
  (`self.E_CrownRotate`))

(event `E_CrownMeshMove`
  ;[1 1 1] 王冠移動
  (`/Engine/EditorBlueprintResources/StandardMacros.DoOnce` false
    (:`Completed`
      (bind _output_get (set `self.FirstCrownLoc` (`SceneComponent.K2_GetComponentLocation` (`self.SM_CrownMesh`))))
      (set `self.FinalCrownLoc` (`KismetMathLibrary.MakeVector` (.x _output_get) (.y _output_get) (.z (`SceneComponent.GetSocketLocation` (`self.MainMesh`) "CrownSocket"))))
      (bind (_direction `_新規track_0`) (`Timeline|タイムライン_0` :!via `PlayFromStart`)
        (:`Update`
          (`SceneComponent.K2_SetRelativeLocation` (`self.SM_CrownMesh`) (`KismetMathLibrary.VLerp` (`self.FirstCrownLoc`) (`self.FinalCrownLoc`) `_新規track_0`) false false))
        (:`Finished`
          (`SceneComponent.K2_AttachToComponent` (`self.SM_CrownMesh`) (`self.MainMesh`) "CrownSocket" "KeepWorld" "KeepWorld" "KeepWorld" true)
          (set `self.CanRotateCrown` false)
          (`self.E_SetNotWait`))))))

(event `E_SetNotWait`
  ;[1 1 1] 待機終了
  (`/Engine/EditorBlueprintResources/StandardMacros.DoOnce` false
    (:`Completed`
      (message `/Game/TeamContent/BP/Player/Result/BPI_ResultCharacterInterface.SetIsWait` (`SkeletalMeshComponent.GetAnimInstance` (`self.MainMesh`)) false)
      (`SceneComponent.K2_SetRelativeLocation` (`self.SM_CrownMesh`) (0.0 3.0 0.0) false false))))

(event `E_CrownRotate`
  ;[1 1 1] 王冠回転
  (if (`self.CanRotateCrown`)
    (`SceneComponent.K2_AddRelativeRotation` (`self.SM_CrownMesh`) (* (`KismetMathLibrary.MakeRotator` 0.0 0.0 1.0) (* (`self.CrownRotateSpeed`) (`GameplayStatics.GetWorldDeltaSeconds`))) false false)))

(fn `GetCrownVisibility`
  (returns (ReturnValue :type Boolean))
  (return (== (`self.Juni`) 0)))

(fn `GetJuni`
  (returns (Juni :type Integer))
  (return (`self.Juni`)))

(fn `UserConstructionScript`
  (bind _mainmesh (`self.MainMesh`))
  (switch `int` (`self.PlayerInde`)
    (:`0`
      (`PrimitiveComponent.SetMaterial` _mainmesh 1 "/Game/TeamContent/Graphic/Mesh/Character/Cloth1P.Cloth1P"))
    (:`1`
      (`PrimitiveComponent.SetMaterial` _mainmesh 1 "/Game/TeamContent/Graphic/Mesh/Character/Cloth2P.Cloth2P"))
    (:`2`
      (`PrimitiveComponent.SetMaterial` _mainmesh 1 "/Game/TeamContent/Graphic/Mesh/Character/Cloth3P.Cloth3P"))
    (:`3`
      (`PrimitiveComponent.SetMaterial` _mainmesh 1 "/Game/TeamContent/Graphic/Mesh/Character/Cloth4P.Cloth4P"))))