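; BP_Human is the playable human character in a multiplayer humans-versus-ghosts game, with per-player materials.
; Fear from GameState gates the cooldown-limited punch, whose box trace damages ghosts, and drives fear effects.
; Nearby rosary makers run an input challenge; a held rosary spawns an effect area.
; Server-to-multicast events handle ghost drag and damage, which turns the victim toward the attacker, zooms the camera, records death points and reports death.
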(event `self.ReceiveBeginPlay`
  ;[0.4766 1 0.9502] BeginPlay
  (`SceneComponent.SetVisibility` (`self.RosaryMesh`) false false)
  (set `self.charaParam` "/Game/TeamContent/DataAsset/DA_HumanCharacterData.DA_HumanCharacterData")
  (set `CharacterMovementComponent.MaxWalkSpeed` (`/Game/TeamContent/BP/Player/InGame/Player/BP_CharactorData.WalkSpeed` (`self.charaParam`)) (`self.CharacterMovement`))
  (`self.ChangeMaterial`)
  (message `/Game/TeamContent/BP/UI/BPI_ToUI.SetWidgetComponetOwner` (`WidgetComponent.GetWidget` (`self.Widget`)) (`self.Index`))
  (`parent.ReceiveBeginPlay`))

(event `ChangeMaterial`
  (bind _mesh (`self.Mesh`))
  (switch `int` (`self.Index`)
    (:`0`
      (`PrimitiveComponent.SetMaterial` _mesh 1 "/Game/TeamContent/Graphic/Material/Chara/M_Human_1P.M_Human_1P"))
    (:`1`
      (`PrimitiveComponent.SetMaterial` _mesh 1 "/Game/TeamContent/Graphic/Material/Chara/M_Human_2P.M_Human_2P"))
    (:`2`
      (`PrimitiveComponent.SetMaterial` _mesh 1 "/Game/TeamContent/Graphic/Material/Chara/M_Human_3P.M_Human_3P"))
    (:`3`
      (`PrimitiveComponent.SetMaterial` _mesh 1 "/Game/TeamContent/Graphic/Material/Chara/M_Human_4P.M_Human_4P"))))

(event `self.ReceiveTick`
  (params (DeltaSeconds :type "Float (single-precision)"))
  ;[1 0.4844 0.4844] Tick
  (`self.E_UpdateAttackDelay` DeltaSeconds)
  (`self.BillBord`)
  (`self.TakeDamage_`)
  (`self.FaerEffect`)
  (bind _newparam (message `/Game/TeamContent/BP/Player/InGame/Human/BPI_HumanFaerGaugeInterface.GetFaerValue` (`GameplayStatics.GetGameState`)))
  (set `self.BeforFaerValue` _newparam)
  (`parent.ReceiveTick` DeltaSeconds))

(event `InputAction|HumanAttackKey`
  (params (Key :type "Key Structure"))
  ;[1 1 1] AttackKeyInput
  (:`Pressed`
    (`self.E_Attack`)))

(event `E_UpdateAttackDelay`
  (params (delta :type "Float (double-precision)"))
  ;[1 1 1] AttackDelay更新
  (if (`self.IsLocallyControlled`)
    (bind _output_get (set `self.NowAttackDelay` (- (`self.NowAttackDelay`) delta)))
    (message `/Game/TeamContent/BP/Player/InGame/Player/BPI_ToPlayerState.ISetAttackDelay` (`Controller.PlayerState` (`GameplayStatics.GetPlayerController` 0)) _output_get)))

(event `/Game/TeamContent/BP/Player/InGame/Human/BPI_HumanInterface.AddHumanDamage`
  (params (nowLoc :type "Vector Structure"))
  ;[1 1 1] AddDamage
  (`self.RoS_AddHumanDamage` nowLoc))

(event `RoS_AddHumanDamage`
  (params (DamageGhostLoc :type "Vector Structure"))
  ;[1 1 1] AddDamage
  (`self.MC_AddHumanDamage` DamageGhostLoc))

(event `MC_AddHumanDamage`
  (params (DamageGhostLoc :type "Vector Structure"))
  ;[1 1 1] AddDamage
  (set `self.DamageGhostLoc` DamageGhostLoc)
  (set `self.IsTakeDamage` true)
  (`NiagaraFunctionLibrary.SpawnSystemAtLocation` "/Game/TeamContent/Graphic/Particle/NPS_OBAttack.NPS_OBAttack" (`self.K2_GetActorLocation`))
  (if (`self.IsLocallyControlled`)
    (`self.DisableInput` (`GameplayStatics.GetPlayerController` 0))))

(event `E_Attack`
  (if (< (`self.NowAttackDelay`) 0.0)
    (`self.ATK`)))

(event `Key|Gamepad_FaceButton_Bottom`
  (params (Key :type "Key Structure"))
  (:`Pressed`
    (`|ExecutionSequence`
      (:`then_0`
        (bind _manager (message `/Game/TeamContent/BP/System/MainGame/BPI_ToGameState.IGetBlockFaerAreaManager` (`GameplayStatics.GetGameState`)))
        (for _array_element (`/Game/TeamContent/BP/Gimmick/BP_BlockFearAreaManager.Areas` _manager)
          (if (< (`KismetMathLibrary.VSize` (- (`self.K2_GetActorLocation` _array_element) (`self.K2_GetActorLocation`))) (`/Game/TeamContent/BP/Gimmick/BP_BlockFearArea.OnSwichRange` _array_element))
            (`/Game/TeamContent/BP/Gimmick/BP_GimickBase.SetBlockFearAreaEnable` _array_element true)))))))

(event `BillBord`
  (`/Engine/EditorBlueprintResources/StandardMacros.IsValid` (`self.Widget1`)
    (:`Is Valid`
      (`SceneComponent.SetVisibility` (`self.Widget1`) (`self.HasRosary`) false))
    (:`Is Not Valid`
      _))
  (`/Engine/EditorBlueprintResources/StandardMacros.IsValid` (`self.Widget`)))

(event `/Game/TeamContent/BP/Player/InGame/Player/BPI_Player.AddScore`
  (params (addValue :type Integer))
  ;[1 1 1] スコア加算
  (`self.E_AddScore` addValue))

(event `E_AddScore`
  (params (Score :type Integer :default 1))
  (set `self.Score` (+ Score (`self.Score`))))

(event `TakeDamage_`
  (if (`self.IsTakeDamage`)
    ;[1 1 1] Ghostの方を向く
    (`|ExecutionSequence`
      (:`then_0`
        (if (not (`self.IsDownOver`))
          (`self.K2_SetActorRotation` (`KismetMathLibrary.MakeRotator` 0.0 0.0 (.yaw (`KismetMathLibrary.RInterpTo` (`self.K2_GetActorRotation`) (`KismetMathLibrary.FindLookAtRotation` (`self.K2_GetActorLocation`) (`self.DamageGhostLoc`)) (`GameplayStatics.GetWorldDeltaSeconds`) 7.0))))
          (`/Engine/EditorBlueprintResources/StandardMacros.DoOnce` false
            (:`Completed`
              (`KismetSystemLibrary.Delay` 0.3)
              (if (`self.IsAlive`)
                (set `self.IsAlive` false)
                (bind _deadhumannum (message `/Game/TeamContent/BP/System/MainGame/BPI_ToGameState.IGetDeadHumanNum` (`GameplayStatics.GetGameState`)))
                (bind _output_get (set `self.Temp_OnDeadPoint` _deadhumannum)) ; 自分より先に死んだ人数に応じたポイント
                (message `/Game/TeamContent/BP/Player/InGame/Player/BPI_ToPlayerState.ISetTempOnDeadPoint` (`Controller.PlayerState` (`GameplayStatics.GetPlayerController` 0)) _output_get)
                (`self.RoS_HumanDead`)
                (`NiagaraFunctionLibrary.SpawnSystemAttached` "/Game/TeamContent/Graphic/Particle/NPS_Star01.NPS_Star01" (`self.CapsuleComponent`) "None" (0.0 0.0 30.0) (struct) "KeepRelativeOffset")
                (set `self.IsDownOver` true)
                (`ActorComponent.K2_DestroyComponent` (`self.Widget`))
                (`ActorComponent.K2_DestroyComponent` (`self.Widget1`))
                (`PrimitiveComponent.SetCollisionObjectType` (`self.CapsuleComponent`) "ECC_GameTraceChannel1")
                (`PrimitiveComponent.SetCollisionObjectType` (`self.Mesh`) "ECC_GameTraceChannel1"))))))
      (:`then_1`
        (`/Engine/EditorBlueprintResources/StandardMacros.DoOnce` false
          (:`Completed`
            (message `/Game/TeamContent/BP/System/MainGame/BPI_ToGameState.ZoomCamera` (`GameplayStatics.GetGameState`) (`SceneComponent.K2_GetComponentLocation` (`self.CapsuleComponent`)) 3.0)))))))

(event `RoS_HumanDead`
  ;[1 1 1] 死亡通知を送信
  (message `/Game/TeamContent/BP/System/MainGame/BPI_ToGameState.IHumanDead` (`GameplayStatics.GetGameState`)))

(event `FaerEffect`
  (bind _newparam (message `/Game/TeamContent/BP/Player/InGame/Human/BPI_HumanFaerGaugeInterface.GetFaerValue` (`GameplayStatics.GetGameState`)))
  (if (< _newparam (`|GetArrayItem` (`/Game/TeamContent/BP/Player/InGame/Player/BP_CharactorData.ActionValue` (`self.charaParam`))))
    (bind _newparam_2 (message `/Game/TeamContent/BP/Player/InGame/Human/BPI_HumanFaerGaugeInterface.GetFaerValue` (`GameplayStatics.GetGameState`)))
    (if (> (- _newparam_2 (`self.BeforFaerValue`)) 0.0)
      (`SceneComponent.SetVisibility` (`self.FaerEffect1`) true false)
      (`SceneComponent.SetVisibility` (`self.FaerEffect2`) false false)
      (else
        (`SceneComponent.SetVisibility` (`self.FaerEffect1`) false false)
        (`SceneComponent.SetVisibility` (`self.FaerEffect2`) false false)))
    (else
      (`SceneComponent.SetVisibility` (`self.FaerEffect1`) true false)
      (`SceneComponent.SetVisibility` (`self.FaerEffect2`) true false))))

(event `/Game/TeamContent/BP/Player/InGame/Human/BPI_HumanInterface.CommitOnDeadPoint`
  ;[1 1 1] おばけ勝利時、自分より先に死んだ人数に応じてポイント加算
  (`self.E_AddScore` (`self.Temp_OnDeadPoint`)))

(event `Key|Gamepad_FaceButton_Bottom`
  (params (Key :type "Key Structure"))
  (:`Pressed`
    (`self.E_ChckRosary`)))

(event `E_ChckRosary`
  ;[1 1 1] ロザリオメーカー起動
  (if (not (`self.IsRosaryPlaying`))
    (`self.E_SerchRosaryMaker`)
    (`self.E_TyrUseRosary`)))

(event `/Game/TeamContent/BP/Player/InGame/Human/BPI_HumanInterface.RosaryPlayEnd`
  ;[1 1 1] ロザリオチャレンジ終了
  (set `self.IsRosaryPlaying` false)
  (set `self.RosaryMakerActor` null))

(event `Key|AnyKey`
  (params (Key :type "Key Structure"))
  (:`Pressed`
    (if (`self.IsRosaryPlaying`)
      (message `/Game/TeamContent/BP/Gimmick/BPI_GimmickInteface.TryInput` (`self.RosaryMakerActor`) Key))))

(event `E_SerchRosaryMaker`
  ;[1 1 1] ロザリオメーカーを探す
  (bind (_outactors _returnvalue) (`KismetSystemLibrary.SphereOverlapActors` (`self.K2_GetActorLocation`) 1000.0 (`|MakeArray` "ObjectTypeQuery1" "ObjectTypeQuery2" :!type "EObjectTypeQuery Enum") "/Game/TeamContent/BP/Gimmick/BP_RosaryMaker.BP_RosaryMaker_C"))
  (if _returnvalue
    (bind _output (`|GetArrayItem` _outactors))
    (bind _playing (message `/Game/TeamContent/BP/Gimmick/BPI_GimmickInteface.IsCanPlay` _output self))
    (if _playing
      (message `/Game/TeamContent/BP/Gimmick/BPI_GimmickInteface.PlayStart` _output self)
      (set `self.RosaryMakerActor` _output)
      (set `self.IsRosaryPlaying` true))))

(event `E_TyrUseRosary`
  (if (`self.HasRosary`)
    (`|SpawnActorFromClass` "/Game/TeamContent/BP/Gimmick/BP_RosaryEffectArea.BP_RosaryEffectArea_C" (`KismetMathLibrary.MakeTransform` (`self.RosaryEffectSpawnLoc`) (struct :`Yaw` 180.0)) "Undefined" "OverrideRootScale" null (`self.EffectTime`) (`self.RosaryEffectRange`) null)
    (`SceneComponent.SetVisibility` (`self.RosaryMesh`) false false)
    (set `self.HasRosary` false)))

(event `/Game/TeamContent/BP/Player/InGame/Human/BPI_HumanInterface.GetRosary`
  (params (EffectRange :type "Float (single-precision)") (Time :type "Float (single-precision)"))
  ;[1 1 1] ロザリオゲット
  (set `self.RosaryEffectRange` EffectRange)
  (set `self.EffectTime` Time)
  (set `self.HasRosary` true)
  (`SceneComponent.SetVisibility` (`self.RosaryMesh`) true false))

(event `RoS_AddDamageToGhost`
  (params (GhostIndex :type Integer) (hitlocation :type "Vector Structure"))
  (message `/Game/TeamContent/BP/Player/InGame/Ghost/BPI_GhostInterface.IAddDamageToGhost` (`GameplayStatics.GetGameState`) GhostIndex hitlocation))

(event `Key|SpaceBar`
  (params (Key :type "Key Structure"))
  (:`Pressed`
    (`self.RoS_GhostDead`)))

(event `RoS_GhostDead`
  (message `/Game/TeamContent/BP/System/MainGame/BPI_ToGameState.IGhostDead` (`GameplayStatics.GetGameState`)))

(event `RoS_Dragmove`
  (params (WorldDirection :type "Vector Structure") (ScaleValue :type "Float (double-precision)") (GhostLoc :type "Vector Structure (by ref)") (GhostRotation :type "Rotator Structure"))
  (`self.MC_Dragmove` ScaleValue GhostLoc GhostRotation))

(event `MC_Dragmove`
  (params (ScaleValue :type "Float (double-precision)") (GhostLocation :type "Vector Structure") (Rotation :type "Rotator Structure"))
  (bind _returnvalue (`KismetMathLibrary.RandomFloatInRange` -20.0 20.0))
  (set `self.IsDragState` true)
  (`self.AddMovementInput` (- GhostLocation (`self.K2_GetActorLocation`)) ScaleValue)
  (`/Engine/EditorBlueprintResources/StandardMacros.DoOnce` false :!label _label
    (:`Completed`
      (if (< (`KismetMathLibrary.Abs` (- (.yaw (`KismetMathLibrary.FindLookAtRotation` GhostLocation (`self.K2_GetActorLocation`))) (.yaw Rotation))) 10.0)
        (`self.LaunchCharacter` (`KismetMathLibrary.MakeVector` _returnvalue _returnvalue 15.0))
        (`KismetSystemLibrary.Delay` 0.2)
        (goto _label :!via `Reset`)))))

(fn `ATK`
  (bind _newparam (message `/Game/TeamContent/BP/Player/InGame/Human/BPI_HumanFaerGaugeInterface.GetFaerValue` (`GameplayStatics.GetGameState`)))
  (if (<= _newparam (`|GetArrayItem` (`/Game/TeamContent/BP/Player/InGame/Player/BP_CharactorData.ActionValue` (`self.charaParam`))))
    (set `self.NowAttackDelay` (`/Game/TeamContent/BP/Player/InGame/Player/BP_CharactorData.AttackDelayTime` (`self.charaParam`)))
    (`self.PlayAnimMontage` "/Game/TeamContent/Graphic/Animation/AM_Attack.AM_Attack")))

(fn `ATK_Trase`
  (bind _returnvalue (`self.K2_GetActorLocation`))
  (bind (_outhit _returnvalue_2) (`KismetSystemLibrary.BoxTraceSingle` _returnvalue (+ _returnvalue (* (`SceneComponent.GetForwardVector` (`self.CapsuleComponent`)) 100.0)) (`self.AttackRange`) (`self.K2_GetActorRotation`) "TraceTypeQuery1"))
  (if _returnvalue_2
    (bind (_bblockinghit _binitialoverlap _time _distance _location _impactpoint _normal _impactnormal _physmat _hitactor) (`GameplayStatics.BreakHitResult` _outhit))
    (if (`self.ActorHasTag` _hitactor "Ghost")
      (bind _ghostindex (message `/Game/TeamContent/BP/Player/InGame/Ghost/BPI_GhostInterface.IGetGhostIndex` _hitactor))
      (`self.RoS_AddDamageToGhost` _ghostindex _impactpoint)
      (bind _ghost (message `/Game/TeamContent/BP/Player/InGame/Ghost/BPI_GhostInterface.IGetPlayerGhost` (`GameplayStatics.GetGameState`)))
      (if (== _ghost _hitactor)
        _))))

(fn `GetHumanFaerGaugeRate`
  (returns (Value :type "Float (double-precision)"))
  (bind _newparam (message `/Game/TeamContent/BP/Player/InGame/Human/BPI_HumanFaerGaugeInterface.GetFaerValue` (`GameplayStatics.GetGameState`)))
  (return (/ _newparam (`/Game/TeamContent/BP/Player/InGame/Player/BP_CharactorData.MaxFearGaugeValue` (`self.charaParam`)))))

(fn `GetIsAlive`
  (returns (isAlive :type Boolean))
  (return (`self.IsAlive`)))

(fn `GetPunchDelayRate`
  (returns (value :type "Float (double-precision)"))
  (bind _returnvalue (`KismetMathLibrary.Abs` (- (/ (`self.NowAttackDelay`) (`/Game/TeamContent/BP/Player/InGame/Player/BP_CharactorData.AttackDelayTime` (`self.charaParam`))) 1.0)))
  (bind _faerstate_ (message `/Game/TeamContent/BP/Player/InGame/Human/BPI_HumanFaerGaugeInterface.GetIsFaerState` (`GameplayStatics.GetGameState`)))
  (if (not _faerstate_)
    (if (> _returnvalue 1.0)
      (return 1.0)
      (else
        (return _returnvalue)))
    (else
      (return 0.0))))

(fn `IsFaerState`
  (returns (value :type Boolean))
  (bind _newparam (message `/Game/TeamContent/BP/Player/InGame/Human/BPI_HumanFaerGaugeInterface.GetFaerValue` (`GameplayStatics.GetGameState`)))
  (return (>= _newparam (`|GetArrayItem` (`/Game/TeamContent/BP/Player/InGame/Player/BP_CharactorData.ActionValue` (`self.charaParam`))))))

(fn `IsHuman?`
  (returns (NewParam :type Boolean))
  (return true))

(fn `OnMoving`
  (`parent.OnMoving`)
  (message `/Game/TeamContent/BP/Gimmick/BPI_GimmickInteface.PlayEnd` (`self.RosaryMakerActor`)))

(fn `RosaryEffectSpawnLoc`
  (returns (Loc :type "Vector Structure"))
  (return (`KismetMathLibrary.MakeVector` (.x (`self.K2_GetActorLocation`)) (.y (`self.K2_GetActorLocation`)) (- (.z (`self.K2_GetActorLocation`)) (* (`CapsuleComponent.CapsuleHalfHeight` (`self.CapsuleComponent`)) 0.5)))))

(fn `UserConstructionScript`
  (`parent.UserConstructionScript`))