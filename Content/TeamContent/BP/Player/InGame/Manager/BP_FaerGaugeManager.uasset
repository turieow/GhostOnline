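; Manager actor that drives a single fear gauge from the state of all human players.
; Each Tick it checks whether any non-downed human is outside the block-fear areas or within fear range of the ghost's location.
; If so, it charges the ghost's skill gauge through a GameState event and raises fear; otherwise fear decays, clamped to data-asset limits.
; Controller rumble plays while fear rises or stays above its threshold, strong above it and weak below.
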(event `self.ReceiveBeginPlay`
  (set `self.NewVar_0` "/Game/TeamContent/DataAsset/DA_HumanCharacterData.DA_HumanCharacterData")
  (bind _returnvalue (`GameplayStatics.GetActorOfClass` "/Game/TeamContent/BP/Player/InGame/Manager/BP_GhostManager.BP_GhostManager_C"))
  (set `self.Manager` _returnvalue)
  (bind _returnvalue_2 (`GameplayStatics.GetActorOfClass` "/Game/TeamContent/BP/Gimmick/BP_BlockFearAreaManager.BP_BlockFearAreaManager_C"))
  (set `self.BlockFearAreaManager` _returnvalue_2)
  (`KismetSystemLibrary.Delay` 0.0)
  (bind _outactors (`GameplayStatics.GetAllActorsOfClass` "/Game/TeamContent/BP/Player/InGame/Human/BP_Human.BP_Human_C"))
  (set `self.Humans` _outactors))

(event `self.ReceiveTick`
  (params (DeltaSeconds :type "Float (single-precision)"))
  (bind _maxfeargaugevalue (`/Game/TeamContent/BP/Player/InGame/Player/BP_CharactorData.MaxFearGaugeValue` (`self.NewVar_0`)))
  (set `self.isAddState` false)
  (for _array_element (`self.Humans`)
    (`/Engine/EditorBlueprintResources/StandardMacros.IsValid` _array_element
      (:`Is Valid`
        (if (not (`/Game/TeamContent/BP/Player/InGame/Human/BP_Human.IsDownOver` _array_element))
          (if (or (not (`/Game/TeamContent/BP/Gimmick/BP_BlockFearAreaManager.IsInArea` (`self.BlockFearAreaManager`) (`self.K2_GetActorLocation` _array_element))) (`KismetMathLibrary.InRange_FloatFloat` (`KismetMathLibrary.VSize` (- (`/Game/TeamContent/BP/Player/InGame/Manager/BP_GhostManager.GhostLocation` (`self.Manager`)) (`self.K2_GetActorLocation` _array_element))) 0.0 (`/Game/TeamContent/BP/Player/InGame/Player/BP_CharactorData.FearRange` (`self.NewVar_0`))))
            (set `self.isAddState` true)
            (break))))))
  (if (`self.isAddState`)
    (`self.RoS_AddGhostSkillValue`)
    (set `self.FaerGaugeValue` (`KismetMathLibrary.FClamp` (+ (`self.FaerGaugeValue`) (* (`/Game/TeamContent/BP/Player/InGame/Player/BP_CharactorData.AddFearGaugeRate` (`self.NewVar_0`)) (`GameplayStatics.GetWorldDeltaSeconds`))) 0.0 _maxfeargaugevalue))
    (`self.FaerFeedBack` :!label _label)
    (else
      (set `self.FaerGaugeValue` (`KismetMathLibrary.FClamp` (- (`self.FaerGaugeValue`) (* (`/Game/TeamContent/BP/Player/InGame/Player/BP_CharactorData.DownFaerGaugeRate` (`self.NewVar_0`)) (`GameplayStatics.GetWorldDeltaSeconds`))) 0.0 _maxfeargaugevalue))
      (bind _value (`self.IsFaerState`))
      (if _value
        (goto _label)))))

(event `RoS_AddGhostSkillValue`
  ;[1 1 1] お化けのスキルゲージをためる
  (message `/Game/TeamContent/BP/Player/InGame/Ghost/BPI_GhostInterface.Add Ghost Skill Gauge` (`GameplayStatics.GetGameState`)))

(fn `GetFaerValue`
  (returns (NewParam :type "Float (double-precision)"))
  (return (`self.FaerGaugeValue`)))

(fn `GetIsFaerState`
  (returns (`faerState?` :type Boolean))
  (return false))

(fn `IsFaerState`
  (returns (value :type Boolean))
  (return (>= (`self.FaerGaugeValue`) (`|GetArrayItem` (`/Game/TeamContent/BP/Player/InGame/Player/BP_CharactorData.ActionValue` (`self.NewVar_0`))))))

(fn `UserConstructionScript`)