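; Manager for the ghost player, handling body swaps, skill gauge, score and damage routing.
; Shuffles ghosts, sorts them by Y position and assigns gamepad keys, then swaps controllers between bodies on a change.
; A spawned reality ghost trails the player ghost and rises on a timeline when control moves to a spawned non-entity ghost.
; Gauge pays for that form change and for switching off random active fear-area lights.
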(event `self.ReceiveBeginPlay`
  ;[1 0.276 0.276] BeginPlay
  (`self.ReloradGhostActors`)
  (`self.ChangeGhostAllocation` (`self.Ghosts`))
  (set `self.charaParam` "/Game/TeamContent/DataAsset/DA_GhostCharacterData.DA_GhostCharacterData")
  (set `self.IsNotEntityState` true)
  (`self.E_CreatReallyGhost`))

(event `self.ReceiveTick`
  (params (DeltaSeconds :type "Float (single-precision)"))
  ;[0.3474 1 0.9102] Tick
  (`self.E_ReallyGhostMove`))

(event `self.ChangeGhost`
  (params (canChange :type "Key Structure") (SelfGhost :type "/Game/TeamContent/BP/Player/InGame/Ghost/BP_Ghost Object Reference"))
  (if true
    (bind (_newparam _value) (`self.ChangeGhostPick` canChange))
    (if _value
      (`self.ChangeGhostFunction` SelfGhost _newparam)
      (`self.ReloradGhostActors`))))

(event `self.ChangeGhostRandomPic`
  (`self.ReloradGhostActors`)
  (`self.ChangeGhostAllocation` (`self.Ghosts`)))

(event `ReloradGhostActors`
  (bind _outactors (`GameplayStatics.GetAllActorsOfClass` "/Game/TeamContent/BP/Player/InGame/Ghost/BP_Ghost.BP_Ghost_C"))
  (bind _output_get (set `self.Ghosts` _outactors))
  (for (_array_element _array_index) _output_get
    (bind _currentgamenum (message `/Game/TeamContent/BP/System/GameInstance/BPI_GameInstanceInterface.GetCurrentGameNum` (`GameplayStatics.GetGameInstance`)))
    (if (< _currentgamenum 4)
      (set `/Game/TeamContent/BP/Player/InGame/Player/BP_Player.Index` _currentgamenum _array_element)
      (else
        (set `/Game/TeamContent/BP/Player/InGame/Player/BP_Player.Index` 0 _array_element)))
    (if (`/Game/TeamContent/BP/Player/InGame/Ghost/BP_Ghost.IsDragState` _array_element)
      (`KismetArrayLibrary.Array_Remove` (`self.Ghosts`) _array_index))))

(event `self.Add Ghost Skill Gauge`
  (bind _maxfeargaugevalue (`/Game/TeamContent/BP/Player/InGame/Player/BP_CharactorData.MaxFearGaugeValue` (`self.charaParam`)))
  (set `self.SkillGaugeValue` (+ (`self.SkillGaugeValue`) (* (`/Game/TeamContent/BP/Player/InGame/Player/BP_CharactorData.AddFearGaugeRate` (`self.charaParam`)) (`GameplayStatics.GetWorldDeltaSeconds`))))
  (if (> (`self.SkillGaugeValue`) _maxfeargaugevalue)
    (set `self.SkillGaugeValue` _maxfeargaugevalue)))

(event `self.ChangeNotEntityState`
  (params (selfActor :type "/Game/TeamContent/BP/Player/InGame/Ghost/BP_Ghost Object Reference"))
  (`self.ReloradGhostActors`)
  (`self.ChangeNotEntityGhost` selfActor))

(event `self.AddGhostScore`
  (params (AddValue :type Integer))
  ;[1 1 1] スコア加算
  (set `self.Score` (+ AddValue (`self.Score`))))

(event `E_CreatReallyGhost`
  (bind _returnvalue (`|SpawnActorFromClass` "/Game/TeamContent/BP/Player/InGame/Ghost/BP_RealityGhost.BP_RealityGhost_C" (`KismetMathLibrary.MakeTransform` (0.0 0.0 0.0)) "Undefined" "OverrideRootScale" null null))
  (set `self.ReallyGhost` _returnvalue))

(event `E_ReallyGhostMove`
  (bind (_returnvalue _returnvalue2) (`self.GetReallyGhostLerpTransform`))
  (if (not (`self.Astralprojecting`))
    (`self.PlayerGhost`
      (:`then`
        (`self.K2_SetActorTransform` (`self.ReallyGhost`) (`KismetMathLibrary.MakeTransform` _returnvalue _returnvalue2) false false))
      (:`else`))))

(event `E_AstralProjection`
  (bind (_reallityghostfirstlocz_x _reallityghostfirstlocz_y _reallityghostfirstlocz_z) (`KismetMathLibrary.BreakVector` (`self.ReallityGhostFirstLocZ`)))
  (bind (_reallityghostfirstlocz_x_2 _reallityghostfirstlocz_y_2) (`KismetMathLibrary.BreakVector` (`self.ReallityGhostFirstLocZ`)))
  (bind _reallyghost (`self.ReallyGhost`))
  (`/Engine/EditorBlueprintResources/StandardMacros.IsValid` _reallyghost
    (:`Is Valid`
      (`/Game/TeamContent/BP/Player/InGame/Ghost/BP_RealityGhost.AddAlfa` _reallyghost)
      (set `self.ReallityGhostFirstLocZ` (`self.K2_GetActorLocation` (`self.ReallyGhost`)))
      (set `self.Astralprojecting` true)
      (bind (_direction `_新規track_0`) (`Timeline|タイムライン_0` :!via `PlayFromStart`)
        (:`Update`
          (`self.K2_SetActorLocation` (`self.ReallyGhost`) (`KismetMathLibrary.MakeVector` _reallityghostfirstlocz_x_2 _reallityghostfirstlocz_y_2 (+ `_新規track_0` _reallityghostfirstlocz_z)) false false))
        (:`Finished`
          (set `self.Astralprojecting` false)
          (`/Game/TeamContent/BP/Player/InGame/Ghost/BP_RealityGhost.DisAlfa` (`self.ReallyGhost`))
          (goto _label :!via `Reset`))))))

(event `self.TrySetGhostMeshVisibility`
  (params (visibility :type Boolean) (actor :type "Actor Object Reference"))
  (bind (_returnvalue _returnvalue2) (`self.GetReallyGhostTransform` actor))
  (if (not (`self.Astralprojecting`))
    (if (not (`/Game/TeamContent/BP/Player/InGame/Ghost/BP_RealityGhost.IsSurprise` (`self.ReallyGhost`)))
      (if visibility
        (`/Engine/EditorBlueprintResources/StandardMacros.DoOnce` false :!label _label
          (:`Completed`
            (`self.K2_SetActorTransform` (`self.ReallyGhost`) (`KismetMathLibrary.MakeTransform` _returnvalue _returnvalue2) false false)
            (`KismetSystemLibrary.DrawDebugSphere` (0.0 0.0 0.0) 100.0 12 (struct :`G` 0.044481 :`B` 1.0 :`A` 1.0) 5.0)
            (`/Game/TeamContent/BP/Player/InGame/Ghost/BP_RealityGhost.AddAlfa` (`self.ReallyGhost`))))
        (else
          (`|ExecutionSequence`
            (:`then_0`
              (goto _label :!via `Reset`))
            (:`then_1`
              (`/Game/TeamContent/BP/Player/InGame/Ghost/BP_RealityGhost.DisAlfa` (`self.ReallyGhost`)))))))))

(event `self.GhostSurprise`
  (`/Game/TeamContent/BP/Player/InGame/Ghost/BP_RealityGhost.Surprise` (`self.ReallyGhost`)))

(event `E_SetGhostLocation`
  (params (GhostLocation :type "Vector Structure"))
  ;[1 1 1] GhostLocation設定
  (set `self.GhostLocation` GhostLocation))

(event `self.TryChangeFoamState`
  (params (Ghost :type "/Game/TeamContent/BP/Player/InGame/Ghost/BP_Ghost Object Reference"))
  (bind _output (`|GetArrayItem` (`/Game/TeamContent/BP/Player/InGame/Player/BP_CharactorData.ActionValue` (`self.charaParam`)) 1))
  (if (not (`self.IsNotEntityState`))
    (if (> (`self.SkillGaugeValue`) _output)
      (set `self.SkillGaugeValue` (- (`self.SkillGaugeValue`) _output))
      (`NiagaraFunctionLibrary.SpawnSystemAttached` "/Game/TeamContent/Graphic/Particle/NPS_Yuutai.NPS_Yuutai" (`Character.Mesh` (`self.PlayerGhost`)) "None" (0.0 0.0 0.0) (struct) "KeepRelativeOffset" true)
      (`self.ChangeNotEntityState` Ghost))))

(event `self.TryDistarb`
  (bind _output (`|GetArrayItem` (`/Game/TeamContent/BP/Player/InGame/Player/BP_CharactorData.ActionValue` (`self.charaParam`)) 2))
  (if (>= (`self.SkillGaugeValue`) _output)
    (set `self.SkillGaugeValue` (- (`self.SkillGaugeValue`) _output))
    (`self.E_TakeOffLight`)))

(event `self.ISetSkillGaugeValue`
  (params (skillGaugeValue :type "Float (single-precision)"))
  (set `self.SkillGaugeValue` skillGaugeValue))

(event `E_TakeOffLight`
  ;[1 1 1] ライトを消す
  (bind _manager (message `/Game/TeamContent/BP/System/MainGame/BPI_ToGameState.IGetBlockFaerAreaManager` (`GameplayStatics.GetGameState`)))
  (bind _areas (`/Game/TeamContent/BP/Gimmick/BP_BlockFearAreaManager.Areas` _manager))
  (bind _output_get (set `self.RandomLightIndex` (`self.TakeRandomIndex` (`/Game/TeamContent/BP/Player/InGame/Player/BP_CharactorData.TurnOffLightNum` (`self.charaParam`)) 0 (`KismetArrayLibrary.Array_LastIndex` _areas) _manager)))
  (for _array_element _output_get
    (message `/Game/TeamContent/BP/Gimmick/BPI_Gimick.SetBlockFearAreaEnable` (`|GetArrayItem` _areas _array_element) false)))

(event `self.IAddDamageToGhost`
  (params (GhostIndex :type Integer) (hitlocation :type "Vector Structure"))
  (for _array_element (`self.Ghosts`)
    (if (== (`/Game/TeamContent/BP/Player/InGame/Ghost/BP_Ghost.GhostIndex` _array_element) GhostIndex)
      (`/Game/TeamContent/BP/Player/InGame/Ghost/BP_Ghost.RoS_AddDamage` _array_element hitlocation))))

(fn `ChangeGhostAllocation`
  (params (NewParam :type "Array of /Game/TeamContent/BP/Player/InGame/Ghost/BP_Ghost Object Reference"))
  (locals (nowCount :type Integer) (changeGhosts0 :type "Array of /Game/TeamContent/BP/Player/InGame/Ghost/BP_Ghost Object Reference") (tmpobj :type "/Game/TeamContent/BP/Player/InGame/Ghost/BP_Ghost Object Reference") (SortCount :type Integer) (localparam :type "Array of /Game/TeamContent/BP/Player/InGame/Ghost/BP_Ghost Object Reference"))
  (bind _localparam (`local.localparam`))
  (bind _changeghosts (`self.ChangeGhosts`))
  (bind _sortcount (`local.SortCount`))
  (bind _returnvalue (- _sortcount 1))
  (bind (_returnvalue_x _returnvalue_y) (`KismetMathLibrary.BreakVector` (`self.K2_GetActorLocation` (`|GetArrayItem` (`self.ChangeGhosts`) (- _sortcount 1)))))
  (set `local.localparam` NewParam)
  (`KismetArrayLibrary.Array_Clear` (`self.ChangeGhosts`)) ; 初期化
  (`KismetArrayLibrary.Array_Clear` (`local.changeGhosts0`))
  (`KismetArrayLibrary.Array_Shuffle` _localparam)
  (for _array_element _localparam
    (set `/Game/TeamContent/BP/Player/InGame/Ghost/BP_Ghost.ChangeKey` (struct) _array_element)
    (if (and (> (`self.GhostValue`) (`local.nowCount`)) (not (`/Game/TeamContent/BP/Player/InGame/Ghost/BP_Ghost.IsDragState` _array_element)))
      (`KismetArrayLibrary.Array_Add` (`local.changeGhosts0`) _array_element)
      (`/Engine/EditorBlueprintResources/StandardMacros.IncrementInt` (`local.nowCount`))))
  (for (_array_element_2 _array_index) (`local.changeGhosts0`)
    (if (<= _array_index 0)
      (`KismetArrayLibrary.Array_Add` (`self.ChangeGhosts`) _array_element_2)
      (else
        (`/Engine/EditorBlueprintResources/StandardMacros.IsValid` _array_element_2
          (:`Is Valid`
            (`KismetArrayLibrary.Array_Add` (`self.ChangeGhosts`) _array_element_2)
            (bind (_arrayindex _arrayelement) (`/Engine/EditorBlueprintResources/StandardMacros.ReverseForEachLoop` (`self.ChangeGhosts`))
              (:`LoopBody`
                (bind _output_get (set `local.SortCount` _arrayindex))
                (if (> _output_get 0)
                  (bind (_returnvalue_x_2 _returnvalue_y_2) (`KismetMathLibrary.BreakVector` (`self.K2_GetActorLocation` _arrayelement)))
                  (if (> _returnvalue_y_2 _returnvalue_y)
                    (set `local.tmpobj` _arrayelement) ; こっから入れ替え処理
                    (`KismetArrayLibrary.Array_Set` _changeghosts _sortcount (`|GetArrayItem` _changeghosts _returnvalue))
                    (`KismetArrayLibrary.Array_Set` _changeghosts _returnvalue (`local.tmpobj`)))))))))))
  (for (_array_element_3 _array_index_2) (`self.ChangeGhosts`)
    (switch `int` _array_index_2 ; 変更キー割り当て
      (:`0`
        (set `/Game/TeamContent/BP/Player/InGame/Ghost/BP_Ghost.ChangeKey` "Gamepad_FaceButton_Right" _array_element_3))
      (:`1`
        (set `/Game/TeamContent/BP/Player/InGame/Ghost/BP_Ghost.ChangeKey` "Gamepad_FaceButton_Bottom" _array_element_3))
      (:`2`
        (set `/Game/TeamContent/BP/Player/InGame/Ghost/BP_Ghost.ChangeKey` "Gamepad_FaceButton_Top" _array_element_3))
      (:`3`
        (set `/Game/TeamContent/BP/Player/InGame/Ghost/BP_Ghost.ChangeKey` "Gamepad_FaceButton_Left" _array_element_3))
      (:`4`
        (set `/Game/TeamContent/BP/Player/InGame/Ghost/BP_Ghost.ChangeKey` "Gamepad_DPad_Right" _array_element_3))
      (:`5`
        (set `/Game/TeamContent/BP/Player/InGame/Ghost/BP_Ghost.ChangeKey` "Gamepad_DPad_Up" _array_element_3))
      (:`6`
        (set `/Game/TeamContent/BP/Player/InGame/Ghost/BP_Ghost.ChangeKey` "Gamepad_DPad_Down" _array_element_3))
      (:`7`
        (set `/Game/TeamContent/BP/Player/InGame/Ghost/BP_Ghost.ChangeKey` "Gamepad_DPad_Left" _array_element_3)))
    (`/Engine/EditorBlueprintResources/StandardMacros.IncrementInt` (`local.nowCount`))))

(fn `ChangeGhostFunction`
  (params (NowGhost :type "/Game/TeamContent/BP/Player/InGame/Ghost/BP_Ghost Object Reference") (NextGhost :type "/Game/TeamContent/BP/Player/InGame/Ghost/BP_Ghost Object Reference"))
  (locals (NewLocalVar_0 :type "Controller Object Reference") (NewLocalVar_1 :type "Transform Structure"))
  (if (not (`KismetStringLibrary.StartsWith` (`KismetSystemLibrary.GetDisplayName` (`Pawn.GetController` NextGhost)) "PlayerController"))
    (bind _asbp_ghost (cast `/Game/TeamContent/BP/Player/InGame/Ghost/BP_Ghost` NowGhost))
    (bind _asbp_ghost_2 (cast `/Game/TeamContent/BP/Player/InGame/Ghost/BP_Ghost` NextGhost))
    ;[1 1 1] PlayerControllerの受け渡し
    (set `local.NewLocalVar_0` (`Pawn.GetController` _asbp_ghost_2))
    (bind _capsulecomponent (`Character.CapsuleComponent` _asbp_ghost_2))
    (set `local.NewLocalVar_1` (`SceneComponent.K2_GetComponentToWorld` _capsulecomponent))
    (`SceneComponent.K2_SetWorldTransform` _capsulecomponent (`KismetMathLibrary.MakeTransform` (0.0 0.0 0.0)) false false) ; Controllerバグるから一回トランスフォームリセット
    (bind _playercontroller (message `/Game/TeamContent/BP/System/GameInstance/BPI_GameInstanceInterface.GetMyPlayerController` (`GameplayStatics.GetGameInstance`) (`/Game/TeamContent/BP/Player/InGame/Player/BP_Player.Index` _asbp_ghost)))
    (`Controller.Possess` _playercontroller _asbp_ghost_2)
    (`SceneComponent.K2_SetWorldTransform` _capsulecomponent (`local.NewLocalVar_1`) false false)
    (`Controller.Possess` (`local.NewLocalVar_0`) _asbp_ghost)
    (bind _state (message `/Game/TeamContent/BP/System/MainGame/BPI_GameModeInterface.GetGameState` (`GameplayStatics.GetGameMode`)))
    (if (`|EnumEquality` _state "NewEnumerator0")
      ;[1 1 1] カメラ再設定
      (bind _returnvalue (`GameplayStatics.GetActorOfClass` "/Game/TeamContent/BP/Gimmick/BP_MainCamera.BP_MainCamera_C"))
      (`PlayerController.SetViewTargetWithBlend` (`GameplayStatics.GetPlayerController` 0) _returnvalue 0.0 "VTBlend_Linear" 0.0 false))))

(fn `ChangeGhostPick`
  (params (Key :type "Key Structure" :default "None"))
  (returns (NewParam :type "/Game/TeamContent/BP/Player/InGame/Ghost/BP_Ghost Object Reference") (value :type Boolean))
  (for _array_element (`self.ChangeGhosts`)
    (if (== (`/Game/TeamContent/BP/Player/InGame/Ghost/BP_Ghost.ChangeKey` _array_element) Key)
      (return _array_element true)))
  (return null false))

(fn `ChangeNotEntityGhost`
  (params (NewParam :type "/Game/TeamContent/BP/Player/InGame/Ghost/BP_Ghost Object Reference"))
  (locals (NoEntGhost :type "/Game/TeamContent/BP/Player/InGame/Ghost/BP_NotEntityGhost Object Reference") (NewLocalVar_3 :type "Controller Object Reference") (NewLocalVar_2 :type "Controller Object Reference"))
  (bind _index (`/Game/TeamContent/BP/Player/InGame/Player/BP_Player.Index` NewParam))
  (bind _playerghost (`self.PlayerGhost`))
  (`/Engine/EditorBlueprintResources/StandardMacros.IsValid` _playerghost
    (:`Is Valid`
      (`self.WalkSlow` _playerghost false))
    (:`Is Not Valid`
      _))
  (`self.E_AstralProjection`)
  (bind _returnvalue (`|SpawnActorFromClass` "/Game/TeamContent/BP/Player/InGame/Ghost/BP_NotEntityGhost.BP_NotEntityGhost_C" (`KismetMathLibrary.MakeTransform` (0.0 0.0 999.0)) "Undefined" "OverrideRootScale" null _index null))
  (set `local.NoEntGhost` _returnvalue)
  (set `local.NewLocalVar_2` (`Pawn.GetController` (`local.NoEntGhost`)))
  (bind _playercontroller (message `/Game/TeamContent/BP/System/GameInstance/BPI_GameInstanceInterface.GetMyPlayerController` (`GameplayStatics.GetGameInstance`) _index))
  (`Controller.Possess` _playercontroller (`local.NoEntGhost`))
  (`Controller.Possess` (`local.NewLocalVar_2`) NewParam)
  (set `self.IsNotEntityState` true)
  (bind _state (message `/Game/TeamContent/BP/System/MainGame/BPI_GameModeInterface.GetGameState` (`GameplayStatics.GetGameMode`)))
  (if (`|EnumEquality` _state "NewEnumerator0")
    ;[1 1 1] カメラ再設定
    (bind _returnvalue_2 (`GameplayStatics.GetActorOfClass` "/Game/TeamContent/BP/Gimmick/BP_MainCamera.BP_MainCamera_C"))
    (`PlayerController.SetViewTargetWithBlend` (`GameplayStatics.GetPlayerController` 0) _returnvalue_2 0.0 "VTBlend_Linear" 0.0 false)
    (`self.ChangeGhostAllocation` (`self.Ghosts`))))

(fn `GetChangeGhost`
  (params (NewParam :type "Key Structure"))
  (returns (NewParam1 :type "/Game/TeamContent/BP/Player/InGame/Ghost/BP_Ghost Object Reference") (NewParam2 :type Boolean))
  (bind (_newparam _value) (`self.ChangeGhostPick` NewParam))
  (return _newparam _value))

(fn `GetGhostFaerGaugeRate`
  (returns (NewParam :type "Float (double-precision)"))
  (return (/ (`self.SkillGaugeValue`) (`/Game/TeamContent/BP/Player/InGame/Player/BP_CharactorData.MaxFearGaugeValue` (`self.charaParam`)))))

(fn `GetGhostManager`
  (returns (NewParam :type "/Game/TeamContent/BP/Player/InGame/Manager/BP_GhostManager Object Reference"))
  (return null))

(fn `GetReallyGhostLerpTransform`
  (returns (ReturnValue :type "Vector Structure") (ReturnValue2 :type "Rotator Structure"))
  (bind _playerghost (`self.PlayerGhost`)
    (:`then`
      (return (`KismetMathLibrary.VLerp` (`self.K2_GetActorLocation` (`self.ReallyGhost`)) (+ (`self.K2_GetActorLocation` _playerghost) (* (* (`self.GetActorForwardVector` (`self.PlayerGhost`)) -1.0) 40.0)) 0.1) (`KismetMathLibrary.RLerp` (`self.K2_GetActorRotation` (`self.ReallyGhost`)) (`self.K2_GetActorRotation` (`self.PlayerGhost`)) 0.1)))
    (:`else`)))

(fn `GetReallyGhostTransform`
  (params (`ターゲット` :type "Actor Object Reference"))
  (returns (ReturnValue :type "Vector Structure") (ReturnValue2 :type "Rotator Structure"))
  (return (+ (`self.K2_GetActorLocation` `ターゲット`) (* (* (`self.GetActorForwardVector` `ターゲット`) -1.0) 40.0)) (`self.K2_GetActorRotation` `ターゲット`)))

(fn `IGetGhostIndex`
  (returns (ghostIndex :type Integer))
  (return 0))

(fn `IGetIsCanChange`
  (returns (NewParam :type Boolean))
  (return false))

(fn `IGetPlayerGhost`
  (returns (ghost :type "/Game/TeamContent/BP/Player/InGame/Ghost/BP_Ghost Object Reference"))
  (return (`self.PlayerGhost`)))

(fn `IGetSkillValue`
  (returns (skillValue :type "Float (double-precision)"))
  (return (`self.SkillGaugeValue`)))

(fn `TakeRandomIndex`
  (params (TakeNum :type Integer) (MinIndex :type Integer) (MaxIndex :type Integer) (NewParam :type "/Game/TeamContent/BP/Gimmick/BP_BlockFearAreaManager Object Reference"))
  (returns (RandomValues :type "Array of Integer"))
  (locals (TakedNum :type Integer) (Min :type Integer) (Max :type Integer) (TakedValue :type "Array of Integer") (random :type Integer :default 0) (LoopNum :type Integer))
  (set `local.Min` MinIndex)
  (set `local.Max` MaxIndex)
  (while (and (> TakeNum (`local.TakedNum`)) (< (`local.LoopNum`) 100))
    (`/Engine/EditorBlueprintResources/StandardMacros.IncrementInt` (`local.LoopNum`)
      (:`  `
        (set `local.random` (`KismetMathLibrary.RandomIntegerInRange` (`local.Min`) (`local.Max`)))
        (if (and (== (`KismetArrayLibrary.Array_Find` (`local.TakedValue`) (`local.random`)) -1) (`/Game/TeamContent/BP/Gimmick/BP_BlockFearAreaManager.GetIsActive` NewParam (`local.random`)))
          (`KismetArrayLibrary.Array_Add` (`local.TakedValue`) (`local.random`))
          (`/Engine/EditorBlueprintResources/StandardMacros.IncrementInt` (`local.TakedNum`))))))
  (return (`local.TakedValue`)))

(fn `UserConstructionScript`)