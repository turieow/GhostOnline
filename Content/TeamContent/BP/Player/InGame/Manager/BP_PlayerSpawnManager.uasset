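; Player spawn manager that replaces controlled pawns with one ghost and the rest humans for the current round.
; E_CreateMainPlayer loops the GameMode's controllers, destroys each existing pawn, then spawns and possesses BP_NotEntityGhost where the index matches the GameState round, otherwise BP_Human.
; Spawn points are SpawnLocation offsets from this actor, and humans are collected in Humans.
; CreateGhost and CreateHuman, with AI ghost fallback, serve only a disconnected older spawn path.
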(event `self.ReceiveBeginPlay`)

(event `E_CreateMainPlayer`
  (set `self.PlayerSpawnCount` 0)
  (bind _round (message `/Game/TeamContent/BP/System/MainGame/BPI_ToGameState.IGetCurrentRound` (`GameplayStatics.GetGameState`)))
  (bind _newparam (message `/Game/TeamContent/BP/System/MainGame/BPI_GameModeInterface.IGetControllersRef` (`GameplayStatics.GetGameMode`)))
  (for (_array_element _array_index) _newparam
    (bind _returnvalue (`Controller.K2_GetPawn` _array_element))
    (`/Engine/EditorBlueprintResources/StandardMacros.IsValid` _returnvalue
      (:`Is Valid`
        (`self.K2_DestroyActor` _returnvalue)
        (if (== _round _array_index)
          (bind _returnvalue_2 (`|SpawnActorFromClass` "/Game/TeamContent/BP/Player/InGame/Ghost/BP_NotEntityGhost.BP_NotEntityGhost_C" (`KismetMathLibrary.MakeTransform` (+ (`|GetArrayItem` (`self.SpawnLocation`)) (`self.K2_GetActorLocation`))) "Undefined" "OverrideRootScale" null _array_index null))
          (`Controller.Possess` _array_element _returnvalue_2)
          (else
            (bind _returnvalue_3 (`|SpawnActorFromClass` "/Game/TeamContent/BP/Player/InGame/Human/BP_Human.BP_Human_C" (`KismetMathLibrary.MakeTransform` (+ (`|GetArrayItem` (`self.SpawnLocation`) (`self.PlayerSpawnCount`)) (`self.K2_GetActorLocation`))) "Undefined" "OverrideRootScale" null _array_index null))
            (`Controller.Possess` _array_element _returnvalue_3)
            (`KismetArrayLibrary.Array_Add` (`self.Humans`) _returnvalue_3)
            (`/Engine/EditorBlueprintResources/StandardMacros.IncrementInt` (`self.PlayerSpawnCount`))))))))

(fn `UserConstructionScript`)