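; Non-entity ghost player for the astral projection state, which lets the player switch back into a ghost form.
; BeginPlay triggers astral projection on BP_GhostManager; Tick reports a far-off ghost location to GameState and enables changing once a delay expires.
; The change key, gated on game status, sends server RPCs for countdown and possession through GameState, clears the manager's non-entity flag, then destroys this actor.
; Ghost getter functions are empty stubs, except the manager getter.
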(event `RoS_SetCountDownFlag`
  (params (iscountDown :type Boolean))
  ;[1 1 1] RoS：カウントダウンフラグを設定
  (`self.MC_SetCountDownFlag` iscountDown))

(event `MC_SetCountDownFlag`
  (params (iscountDown :type Boolean))
  ;[1 1 1] RoS：カウントダウンフラグを設定
  (message `/Game/TeamContent/BP/System/MainGame/BPI_ToGameState.ISetCountDownFlag` (`GameplayStatics.GetGameState`) iscountDown))

(event `self.ReceiveBeginPlay`
  (bind _manager (`self.Manager`))
  (bind _returnvalue (`GameplayStatics.GetActorOfClass` "/Game/TeamContent/BP/Player/InGame/Manager/BP_GhostManager.BP_GhostManager_C"))
  (set `self.manager` _returnvalue)
  (set `self.NewVar_0` "/Game/TeamContent/DataAsset/DA_GhostCharacterData.DA_GhostCharacterData")
  (`self.RoS_SetCountDownFlag` false)
  (set `self.NowChangeDelay` (`self.ChangeDelay`))
  (`/Engine/EditorBlueprintResources/StandardMacros.IsValid` _manager
    (:`Is Valid`
      (`/Game/TeamContent/BP/Player/InGame/Manager/BP_GhostManager.E_AstralProjection` _manager))))

(event `Key|AnyKey`
  (params (Key :type "Key Structure")))

(event `InputEvent_ChangeFoamKey`
  (params (NewParam :type "Key Structure" :default "None"))
  (bind _status (message `/Game/TeamContent/BP/System/MainGame/BPI_ToGameState.IGetCurrentGameStatus` (`GameplayStatics.GetGameState`)))
  (if (`|EnumEquality` _status "NewEnumerator0")
    (bind _newparam1 (`self.changeFoam` NewParam))
    (if _newparam1
      (`self.K2_DestroyActor` :!label _label))))

(event `InputAction|ChangeFoamKey`
  (params (Key :type "Key Structure"))
  (:`Pressed`
    (bind _status (message `/Game/TeamContent/BP/System/MainGame/BPI_ToGameState.IGetCurrentGameStatus` (`GameplayStatics.GetGameState`)))
    (if (`|EnumEquality` _status "NewEnumerator0")
      (bind _newparam1 (`self.changeFoam` Key))
      (if _newparam1
        (goto _label)))))

(event `self.ReceiveTick`
  (params (DeltaSeconds :type "Float (single-precision)"))
  (message `/Game/TeamContent/BP/Player/InGame/Ghost/BPI_GhostInterface.ISetGhostLocation` (`GameplayStatics.GetGameState`) (99999.0 99999.0 99999.0))
  (bind _output_get (set `self.NowChangeDelay` (- (`self.NowChangeDelay`) (`GameplayStatics.GetWorldDeltaSeconds`))))
  (if (< _output_get 0.0)
    (message `/Game/TeamContent/BP/Player/InGame/Ghost/BPI_GhostInterface.ISetIsCanChange` (`GameplayStatics.GetGameState`) true)))

(event `RoS_PossessToGhost`
  (params (NewParam :type "Key Structure" :default "None"))
  (message `/Game/TeamContent/BP/Player/InGame/Ghost/BPI_GhostInterface.IChangeGhost` (`GameplayStatics.GetGameState`) NewParam))

(fn `changeFoam`
  (params (NewParam :type "Key Structure" :default "None"))
  (returns (NewParam1 :type Boolean))
  (locals (NewLocalVar_1 :type "Transform Structure"))
  (`self.RoS_SetCountDownFlag` true) ; クライアントの時、ここでやらないと通らない
  (`self.RoS_PossessToGhost` NewParam)
  (set `/Game/TeamContent/BP/Player/InGame/Manager/BP_GhostManager.IsNotEntityState` false (`self.manager`))
  (bind _status (message `/Game/TeamContent/BP/System/MainGame/BPI_ToGameState.IGetCurrentGameStatus` (`GameplayStatics.GetGameState`)))
  (if (`|EnumEquality` _status "NewEnumerator0")
    (`self.RoS_SetCountDownFlag` true)
    (message `/Game/TeamContent/BP/Player/InGame/Ghost/BPI_GhostInterface.ISetIsCanChange` (`GameplayStatics.GetGameState`) false)
    (return true)))

(fn `GetChangeGhost`
  (params (NewParam :type "Key Structure"))
  (returns (NewParam1 :type "/Game/TeamContent/BP/Player/InGame/Ghost/BP_Ghost Object Reference") (NewParam2 :type Boolean))
  (return null false))

(fn `GetGhostCharaParam`
  (returns (CharacterData :type "/Game/TeamContent/BP/Player/InGame/Player/BP_CharactorData Object Reference"))
  (return null))

(fn `GetGhostManager`
  (returns (NewParam :type "/Game/TeamContent/BP/Player/InGame/Manager/BP_GhostManager Object Reference"))
  (return (`self.manager`)))

(fn `GetGhostSkillGaugeRate`
  (returns (NewParam :type "Float (double-precision)"))
  (return 0.0))

(fn `IGetGhostIndex`
  (returns (ghostIndex :type Integer))
  (return 0))

(fn `IGetIsCanChange`
  (returns (NewParam :type Boolean))
  (return false))

(fn `IGetPlayerGhost`
  (returns (ghost :type "/Game/TeamContent/BP/Player/InGame/Ghost/BP_Ghost Object Reference"))
  (return null))

(fn `IGetSkillValue`
  (returns (skillValue :type "Float (double-precision)"))
  (return 0.0))

(fn `UserConstructionScript`)