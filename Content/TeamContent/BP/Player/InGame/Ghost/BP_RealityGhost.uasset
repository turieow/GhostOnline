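; BP_RealityGhost is a ghost actor that starts invisible, fades in and out, and can play a surprise effect.
; Dynamic body and eye materials share an Opacity parameter driven by two timelines.
; Surprise plays a montage and sets a flag; Tick then runs a timeline animating opacity and mesh scale, then hides the ghost.
; AddAlfa and DisAlfa drive the fade timeline forward or backward through DoOnce gates, ignored during a surprise.
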(event `self.ReceiveBeginPlay`
  (bind _returnvalue (`PrimitiveComponent.CreateDynamicMaterialInstance` (`self.SK_Ghost`) 0 "/Game/TeamContent/Graphic/Mesh/Character/Ghost.Ghost" "None"))
  (bind _output_get (set `self.BodyMaterial` _returnvalue))
  (`PrimitiveComponent.SetMaterial` (`self.SK_Ghost`) 0 _output_get)
  (bind _returnvalue_2 (`PrimitiveComponent.CreateDynamicMaterialInstance` (`self.SK_Ghost`) 1 "/Game/TeamContent/Graphic/Mesh/Character/Ghost_Eye.Ghost_Eye" "None"))
  (bind _output_get_2 (set `self.EyeMaterial` _returnvalue_2))
  (`PrimitiveComponent.SetMaterial` (`self.SK_Ghost`) 1 _output_get_2)
  (`MaterialInstanceDynamic.SetScalarParameterValue` (`self.BodyMaterial`) "Opacity" 0.0)
  (`MaterialInstanceDynamic.SetScalarParameterValue` (`self.EyeMaterial`) "Opacity" 0.0))

(event `self.ReceiveTick`
  (params (DeltaSeconds :type "Float (single-precision)"))
  (if (`self.IsSurprise`)
    (`/Engine/EditorBlueprintResources/StandardMacros.DoOnce` false :!label _label
      (:`Completed`
        (bind (_direction `_新規track_0` `_新規track_1`) (`Timeline|alfa` :!label _label_2)
          (:`Update`
            (`MaterialInstanceDynamic.SetScalarParameterValue` (`self.BodyMaterial`) "Opacity" `_新規track_0`)
            (`MaterialInstanceDynamic.SetScalarParameterValue` (`self.EyeMaterial`) "Opacity" `_新規track_0`)
            (`SceneComponent.SetWorldScale3D` (`self.SK_Ghost`) (`KismetMathLibrary.MakeVector` `_新規track_1` `_新規track_1` `_新規track_1`)))
          (:`Finished`
            (`|ExecutionSequence`
              (:`then_0`
                (goto _label_2 :!via `SetNewTime`))
              (:`then_1`
                (set `self.IsSurprise` false)
                (`KismetSystemLibrary.Delay` 0.0)
                (`MaterialInstanceDynamic.SetScalarParameterValue` (`self.BodyMaterial`) "Opacity" 0.0)
                (`MaterialInstanceDynamic.SetScalarParameterValue` (`self.EyeMaterial`) "Opacity" 0.0)
                (goto _label :!via `Reset`)))))))
    (else
      (`SceneComponent.SetWorldScale3D` (`self.SK_Ghost`) (1.0 1.0 1.0)))))

(event `AddAlfa`
  (if (not (`self.IsSurprise`))
    (`|ExecutionSequence`
      (:`then_0`
        (`/Engine/EditorBlueprintResources/StandardMacros.DoOnce` false :!label _label_3
          (:`Completed`
            (bind (_direction `_新規track_0`) (`Timeline|Alfaff` :!label _label_4)
              (:`Update`
                (`MaterialInstanceDynamic.SetScalarParameterValue` (`self.BodyMaterial`) "Opacity" `_新規track_0`)
                (`MaterialInstanceDynamic.SetScalarParameterValue` (`self.EyeMaterial`) "Opacity" `_新規track_0`))))))
      (:`then_1`
        (goto _label_5 :!via `Reset`)))))

(event `DisAlfa`
  (if (not (`self.IsSurprise`))
    (`|ExecutionSequence`
      (:`then_0`
        (`/Engine/EditorBlueprintResources/StandardMacros.DoOnce` false :!label _label_5
          (:`Completed`
            (goto _label_4 :!via `Reverse`))))
      (:`then_1`
        (goto _label_3 :!via `Reset`)))))

(fn `Surprise`
  (`SkeletalMeshComponent.PlayAnimation` (`self.SK_Ghost`) "/Game/TeamContent/Graphic/Animation/AM_Gost.AM_Gost" false)
  (set `self.IsSurprise` true)
  (return))

(fn `UserConstructionScript`)