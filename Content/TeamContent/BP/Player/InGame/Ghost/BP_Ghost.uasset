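; Ghost character: a plush-bear body, randomly patterned and accessorized, that a player can possess to scare humans.
; Attacks spend skill gauge on humans passing fear, range and angle checks, damaging them, scoring and starting a Tick-driven drag.
; Hits ragdoll and destroy non-dragging bodies, reporting death if possessed; light swaps materials and toggles possessed-ghost visibility.
; Shared state and form changes route through GameState, using server-RPC/multicast pairs for replication.
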(event `self.ReceiveBeginPlay`
  ;[1 0.3698 0.3753] BeginPlay
  (set `self.charaParam` "/Game/TeamContent/DataAsset/DA_GhostCharacterData.DA_GhostCharacterData")
  (set `CharacterMovementComponent.MaxWalkSpeed` (`/Game/TeamContent/BP/Player/InGame/Player/BP_CharactorData.WalkSpeed` (`self.charaParam`)) (`self.CharacterMovement`))
  (bind _outactors (`GameplayStatics.GetAllActorsOfClass` "/Game/TeamContent/BP/Player/InGame/Human/BP_Human.BP_Human_C"))
  (set `self.Humans` _outactors)
  (`self.SetOrnaments`)
  (`PrimitiveComponent.CreateDynamicMaterialInstance` (`self.Mesh`) 0 null "None")
  (`self.RandMaterial`)
  (`parent.ReceiveBeginPlay`))

(event `RandMaterial`
  (switch `int` (`KismetMathLibrary.RandomIntegerInRange` 1 3)
    (:`1`
      (bind _returnvalue (`KismetMaterialLibrary.CreateDynamicMaterialInstance` "/Game/TeamContent/Graphic/Material/Chara/MI_Patarm/MI_BearPatarn01.MI_BearPatarn01"))
      (set `self.MaterialDynamic` _returnvalue)
      (set `self.MaterialValue` 1))
    (:`2`
      (bind _returnvalue_2 (`KismetMaterialLibrary.CreateDynamicMaterialInstance` "/Game/TeamContent/Graphic/Material/Chara/MI_Patarm/MI_BearPatarn02.MI_BearPatarn02"))
      (set `self.MaterialDynamic` _returnvalue_2)
      (set `self.MaterialValue` 2))
    (:`3`
      (bind _returnvalue_3 (`KismetMaterialLibrary.CreateDynamicMaterialInstance` "/Game/TeamContent/Graphic/Material/Chara/MI_Patarm/MI_BearPatarn03.MI_BearPatarn03"))
      (set `self.MaterialDynamic` _returnvalue_3)
      (set `self.MaterialValue` 3)))
  (`PrimitiveComponent.SetMaterial` (`self.Mesh`) 0 (`self.MaterialDynamic`))
  (`PrimitiveComponent.SetMaterial` (`self.Mesh`) 1 (`self.MaterialDynamic`)))

(event `self.ReceiveTick`
  (params (DeltaSeconds :type "Float (single-precision)"))
  ;[0.3021 1 0.7561] Tick
  (`self.WidgetBillBord`)
  (set `self.NowAtkDelay` (- (`self.NowAtkDelay`) DeltaSeconds))
  (`self.NowGhostInfo`)
  (`self.DrawWiget`)
  (`self.DragStateEvent`)
  (`parent.ReceiveTick` DeltaSeconds))

(event `WidgetBillBord`
  ;[1 1 1] TextBillbord
  (`/Engine/EditorBlueprintResources/StandardMacros.IsValid` (`self.Widget`)
    (:`Is Valid`
      (`SceneComponent.K2_SetWorldRotation` (`self.Widget`) (`KismetMathLibrary.FindLookAtRotation` (`self.K2_GetActorLocation`) (`PlayerCameraManager.GetCameraLocation` (`GameplayStatics.GetPlayerCameraManager` 0))) false false)
      (message `/Game/TeamContent/BP/UI/BPI_ToUI.SetKeyImage` (`WidgetComponent.GetWidget` (`self.Widget`)) (`self.ChangeKey`)))))

(event `RoS_SetIsTransfered`
  (params (IsTransfered :type Boolean))
  ;[1 1 1] 乗り移りフラグを設定
  (`self.MC_SEtIsTransfered` IsTransfered))

(event `NowGhostInfo`
  ;[1 1 1] FearArea
  (bind _output_get (set `self.IsTransfered` (`self.IsTransfered`)))
  (if _output_get
    (message `/Game/TeamContent/BP/Player/InGame/Ghost/BPI_GhostInterface.ISetGhostLocation` (`GameplayStatics.GetGameState`) (`self.K2_GetActorLocation`))
    (message `/Game/TeamContent/BP/Player/InGame/Ghost/BPI_GhostInterface.ISetGhostPlayer` (`GameplayStatics.GetGameState`) self)))

(event `MC_SetIsTransfered`
  (params (IsTransfered :type Boolean))
  ;[1 1 1] 乗り移りフラグを設定
  (set `self.IsTransfered` IsTransfered))

(event `RoS_AddDamageToGhost`
  (params (Location :type "Vector Structure"))
  ;[1 1 1] AddDamage
  (`self.MC_AddDamageToGhost` Location))

(event `/Game/TeamContent/BP/Player/InGame/Ghost/BPI_GhostInterface.AddDamage`
  (params (HitLocation :type "Vector Structure"))
  (`KismetSystemLibrary.PrintString` "使われてないものが呼ばれた" true true (struct :`R` 0.243605 :`G` 1.0 :`A` 1.0) 10.0))

(event `MC_AddDamageToGhost`
  (params (Location :type "Vector Structure"))
  (bind _mesh (`self.Mesh`))
  (bind _returnvalue (`SceneComponent.K2_GetComponentLocation` (`self.Mesh`)))
  ;[1 1 1] AddDamage
  (if (not (`self.IsDragState`))
    (set `self.IsTakeDamage` true)
    (`NiagaraFunctionLibrary.SpawnSystemAtLocation` "/Game/TeamContent/Graphic/Particle/NPS_Hit01.NPS_Hit01" Location)
    (`PrimitiveComponent.SetCollisionEnabled` _mesh "QueryAndPhysics")
    (`PrimitiveComponent.SetCollisionResponseToChannel` _mesh "ECC_Pawn" "ECR_Ignore")
    (`SkeletalMeshComponent.SetAllBodiesSimulatePhysics` _mesh true)
    (`PrimitiveComponent.SetCollisionEnabled` (`self.CapsuleComponent`) "NoCollision")
    (`PrimitiveComponent.AddImpulse` _mesh (+ (* (- (`self.K2_GetActorLocation`) Location) 750.0) (0.0 0.0 5000.0)) "None" false)
    (`ActorComponent.K2_DestroyComponent` (`self.Widget`))
    (if (not (`self.IsTransfered`))
      (`KismetSystemLibrary.Delay` 2.0)
      (`NiagaraFunctionLibrary.SpawnSystemAtLocation` "/Game/TeamContent/Graphic/Particle/NPS_NuigurumiEnd.NPS_NuigurumiEnd" (`SceneComponent.K2_GetComponentLocation` (`self.Mesh`)))
      (`self.K2_DestroyActor`)
      (message `/Game/TeamContent/BP/Player/InGame/Ghost/BPI_GhostInterface.ChangeGhostRandomPic` (`GameplayStatics.GetGameState`))
      (else
        (message `/Game/TeamContent/BP/System/MainGame/BPI_ToGameState.ZoomCamera` (`GameplayStatics.GetGameState`) (`self.K2_GetActorLocation`) 1.0)
        (message `/Game/TeamContent/BP/Player/InGame/Ghost/BPI_GhostInterface.ChangeNotEntityState` (`GameplayStatics.GetGameState`) self)
        (`KismetSystemLibrary.Delay` 1.0)
        (`NiagaraFunctionLibrary.SpawnSystemAtLocation` "/Game/TeamContent/Graphic/Particle/NPS_Tyakuti.NPS_Tyakuti" _returnvalue)
        (`KismetSystemLibrary.Delay` 1.0)
        (`NiagaraFunctionLibrary.SpawnSystemAtLocation` "/Game/TeamContent/Graphic/Particle/NPS_NuigurumiEnd.NPS_NuigurumiEnd" _returnvalue)
        (`self.RoS_GhostDead`)
        (`self.K2_DestroyActor`)
        (message `/Game/TeamContent/BP/Player/InGame/Ghost/BPI_GhostInterface.ChangeGhostRandomPic` (`GameplayStatics.GetGameState`))))))

(event `RoS_GhostDead`
  ;[1 1 1] RoS:GameStateにお化け死亡通知を送る
  (message `/Game/TeamContent/BP/System/MainGame/BPI_ToGameState.IGhostDead` (`GameplayStatics.GetGameState`)))

(event `RoS_AddDamageToPlayer`
  (params (human :type "Object Object Reference"))
  (message `/Game/TeamContent/BP/Player/InGame/Human/BPI_HumanInterface.AddHumanDamage` human (`self.K2_GetActorLocation`)))

(event `/Game/TeamContent/BP/Player/InGame/Ghost/BPI_GhostInterface.SetCleanBodyState`
  (params (value :type Boolean))
  (set `self.IsCleanBody` value))

(event `DrawWiget`
  (bind _widget (`self.Widget`))
  (`/Engine/EditorBlueprintResources/StandardMacros.IsValid` (`self.Widget`)
    (:`Is Valid`
      (bind _newparam (message `/Game/TeamContent/BP/Player/InGame/Ghost/BPI_GhostInterface.IGetIsCanChange` (`GameplayStatics.GetGameState`)))
      (if _newparam
        (`SceneComponent.SetVisibility` _widget true false)
        (else
          (`SceneComponent.SetVisibility` _widget false false))))))

(event `E_AddScore`
  (params (AddValue :type Integer :default 1))
  ;[1 1 1] スコア加算
  (message `/Game/TeamContent/BP/Player/InGame/Player/BPI_ToPlayerState.IAddPlayerScore` (`Controller.PlayerState` (`GameplayStatics.GetPlayerController` 0)) AddValue))

(event `/Game/TeamContent/BP/Player/InGame/Player/BPI_Player.AddScore`
  (params (addValue :type Integer))
  ;[1 1 1] スコア加算
  (`self.E_AddScore` addValue))

(event `DragStateEvent`
  (if (`self.IsDragState`)
    (bind _output_get (set `self.AnimDelay` (- (`self.AnimDelay`) (`GameplayStatics.GetWorldDeltaSeconds`))))
    (if (< _output_get 0.0)
      (`|ExecutionSequence`
        (:`then_0`
          (`/Engine/EditorBlueprintResources/StandardMacros.DoOnce` false
            (:`Completed`
              (message `/Game/TeamContent/BP/Player/InGame/Ghost/BPI_GhostInterface.ChangeNotEntityState` (`GameplayStatics.GetGameState`) self))))
        (:`then_1`
          (set `self.ChangeKey` "None") ; RoSのほうがいいかも
          (set `self.ATKHitDragDelay` (- (`self.ATKHitDragDelay`) (`GameplayStatics.GetWorldDeltaSeconds`)))
          (if (< (`self.ATKHitDragDelay`) 0.0)
            (`|ExecutionSequence`
              (:`then_0`
                (`/Engine/EditorBlueprintResources/StandardMacros.DoOnce` false
                  (:`Completed`
                    (`SceneComponent.K2_AddLocalRotation` (`self.Mesh`) (struct :`Yaw` 180.0) false false))))
              (:`then_1`
                (set `self.NowDrag` true)
                (for _array_element (`self.HitHumanIndex`)
                  (`self.RoS_HumanMove` _array_element (0.0 0.0 0.0) 100.0 (`SceneComponent.K2_GetComponentLocation` (`self.Scene`)) (`self.K2_GetActorRotation`)))))
            (else
              (bind _newparam (`self.ABSHitHumanLoc`))
              (if (> (`KismetMathLibrary.VSize` (- _newparam (`self.K2_GetActorLocation`))) 70.0)
                _))))))))

(event `RoS_SetGhostSkillValue`
  (params (skillGaugeValue :type "Float (double-precision)"))
  ;[1 1 1] スキルゲージの値を設定
  (message `/Game/TeamContent/BP/Player/InGame/Ghost/BPI_GhostInterface.ISetSkillGaugeValue` (`GameplayStatics.GetGameState`) skillGaugeValue))

(event `RoS_AddHitHumanIndex`
  (params (NewItem :type "Integer (by ref)"))
  ;[1 1 1] HitHumanIndex　追加
  (`self.MC_AddHitHumanIndex` NewItem))

(event `MC_AddHitHumanIndex`
  (params (NewItem :type "Integer (by ref)"))
  ;[1 1 1] HitHumanIndex　追加
  (`KismetArrayLibrary.Array_Add` (`self.HitHumanIndex`) NewItem))

(event `RoS_HumanMove`
  (params (Index :type Integer) (worldDirection :type "Vector Structure") (scallCalue :type "Float (double-precision)") (GhostLoc :type "Vector Structure") (GhostRot :type "Rotator Structure"))
  ;[1 1 1] 脅かした人間を引きずる
  (message `/Game/TeamContent/BP/Player/InGame/Manager/BPI_ToPlayerSpawnManager.IDragMoveHuman` (`GameplayStatics.GetGameState`) Index worldDirection scallCalue GhostLoc GhostRot))

(event `RoS_SetIsDragState`
  (params (IsDragState :type Boolean))
  (`self.MC_SetISDragState` IsDragState))

(event `MC_SetISDragState`
  (params (IsDragState :type Boolean))
  (set `self.IsDragState` IsDragState))

(event `InputEvent_DisturbKey`
  (`self.RoS_TryDistarb` :!label _label))

(event `RoS_TryDistarb`
  (message `/Game/TeamContent/BP/Player/InGame/Ghost/BPI_GhostInterface.TryDistarb` (`GameplayStatics.GetGameState`)))

(event `InputAction|DisturbKey`
  (params (Key :type "Key Structure"))
  (:`Pressed`
    (goto _label)))

(event `InputEvent_AttackKey`
  ;[1 1 1] AttackKey
  (if (< (`self.NowAtkDelay`) 0.0) :!label _label_2
    (bind _atk (`self.ATK`))
    (if _atk
      (`KismetSystemLibrary.Delay` 0.3)
      (set `self.AnimDelay` (+ (`self.AnimDelay`) 0.85))
      (message `/Game/TeamContent/BP/Player/InGame/Ghost/BPI_GhostInterface.GhostSurprise` (`GameplayStatics.GetGameState`)))))

(event `InputAction|GhostAttackKey`
  (params (Key :type "Key Structure"))
  ;[1 1 1] AttackKey
  (:`Pressed`
    (goto _label_2)))

(event `InputEvent_ChangeFoamStateKey`
  ;[1 1 1] ChangeForm
  (`self.RoS_TryChangeFoamState` :!label _label_3))

(event `InputAction|ChangeFoamStateKey`
  (params (Key :type "Key Structure"))
  ;[1 1 1] ChangeForm
  (:`Pressed`
    (goto _label_3)))

(event `RoS_TryChangeFoamState`
  ;[1 1 1] RoS:幽体離脱
  (message `/Game/TeamContent/BP/Player/InGame/Ghost/BPI_GhostInterface.TryChangeFoamState` (`GameplayStatics.GetGameState`) self))

(event `/Game/TeamContent/BP/Player/InGame/Ghost/BPI_GhostInterface.InLight`
  (bind _mesh (`self.Mesh`))
  (switch `int` (`self.MaterialValue`)
    (:`1`
      (`PrimitiveComponent.SetMaterial` _mesh 1 "/Game/TeamContent/Graphic/Material/Chara/MI_BaseTranse.MI_BaseTranse"))
    (:`2`
      (`PrimitiveComponent.SetMaterial` _mesh 1 "/Game/TeamContent/Graphic/Material/Chara/MI_Patarm/MI_BearTranse02.MI_BearTranse02"))
    (:`3`
      (`PrimitiveComponent.SetMaterial` _mesh 1 "/Game/TeamContent/Graphic/Material/Chara/MI_Patarm/MI_BearTranse03.MI_BearTranse03")))
  (if (`self.IsTransfered`)
    (message `/Game/TeamContent/BP/Player/InGame/Ghost/BPI_GhostInterface.TrySetGhostMeshVisibility` (`GameplayStatics.GetGameState`) true self)))

(event `/Game/TeamContent/BP/Player/InGame/Ghost/BPI_GhostInterface.OutLight`
  (bind _mesh (`self.Mesh`))
  (switch `int` (`self.MaterialValue`)
    (:`1`
      (`PrimitiveComponent.SetMaterial` _mesh 1 "/Game/TeamContent/Graphic/Material/Chara/MI_Patarm/MI_BearPatarn01.MI_BearPatarn01"))
    (:`2`
      (`PrimitiveComponent.SetMaterial` _mesh 1 "/Game/TeamContent/Graphic/Material/Chara/MI_Patarm/MI_BearPatarn02.MI_BearPatarn02"))
    (:`3`
      (`PrimitiveComponent.SetMaterial` _mesh 1 "/Game/TeamContent/Graphic/Material/Chara/MI_Patarm/MI_BearPatarn03.MI_BearPatarn03")))
  (if (`self.IsTransfered`)
    (message `/Game/TeamContent/BP/Player/InGame/Ghost/BPI_GhostInterface.TrySetGhostMeshVisibility` (`GameplayStatics.GetGameState`) false self)))

(event `/Game/TeamContent/BP/Player/InGame/Ghost/BPI_GhostInterface.WalkSlow`
  (params (slow :type Boolean))
  (bind _charaparam (`self.charaParam`))
  (if slow
    (if (`self.IsTransfered`)
      (set `CharacterMovementComponent.MaxWalkSpeed` (`/Game/TeamContent/BP/Player/InGame/Player/BP_CharactorData.SlowWalkSpeed` _charaparam) (`self.CharacterMovement`)))
    (else
      (set `CharacterMovementComponent.MaxWalkSpeed` (`/Game/TeamContent/BP/Player/InGame/Player/BP_CharactorData.WalkSpeed` _charaparam) (`self.CharacterMovement`)))))

(event `Key|A`
  (params (Key :type "Key Structure"))
  (:`Pressed`
    (bind _characterdata (message `/Game/TeamContent/BP/Player/InGame/Ghost/BPI_GhostInterface.GetGhostCharaParam` (`GameplayStatics.GetGameState`)))
    (`self.RoS_SetGhostSkillValue` (`/Game/TeamContent/BP/Player/InGame/Player/BP_CharactorData.MaxFearGaugeValue` _characterdata))))

(event `RoS_ChangeCollisionObjectType`
  (`self.MC_ChangeCollisionObjectType`))

(event `MC_ChangeCollisionObjectType`
  (`PrimitiveComponent.SetCollisionObjectType` (`self.CapsuleComponent`) "ECC_GameTraceChannel1")
  (`PrimitiveComponent.SetCollisionObjectType` (`self.Mesh`) "ECC_GameTraceChannel1"))

(fn `ABSHitHumanLoc`
  (returns (NewParam :type "Vector Structure"))
  (locals (NewLocalVar_0 :type "Vector Structure"))
  (bind _hithumans (`self.HitHumans`))
  (for _array_element _hithumans
    (set `local.NewLocalVar_0` (+ (`self.K2_GetActorLocation` _array_element) (`local.NewLocalVar_0`))))
  (return (/ (`local.NewLocalVar_0`) (`KismetArrayLibrary.Array_Length` _hithumans))))

(fn `ATK`
  (returns (atk :type Boolean))
  (locals (IsCanHitPlayer :type Boolean) (IsHitPlayer :type Boolean) (tmpVector :type "Vector Structure") (LocalHuman :type "Array of /Game/TeamContent/BP/Player/InGame/Human/BP_Human Object Reference"))
  (bind _playerarray (`GameStateBase.PlayerArray` (`GameplayStatics.GetGameState`)))
  (bind _output (`|GetArrayItem` (`/Game/TeamContent/BP/Player/InGame/Player/BP_CharactorData.ActionValue` (`self.charaParam`))))
  ;[1 1 1] 一定範囲内に攻撃可能なPlayerは存在するか判定
  (for _index (range 4)
    ;;[1 1 1] 人間配列を作成
    (if (`KismetArrayLibrary.Array_IsValidIndex` _playerarray _index)
      (bind _asbp_human (cast `/Game/TeamContent/BP/Player/InGame/Human/BP_Human` (`PlayerState.PawnPrivate` (`|GetArrayItem` _playerarray _index))))
      (`KismetArrayLibrary.Array_Add` (`local.LocalHuman`) _asbp_human)
      (bind _newparam (message `/Game/TeamContent/BP/Player/InGame/Human/BPI_HumanFaerGaugeInterface.GetFaerValue` (`GameplayStatics.GetGameState`)))
      (if (>= _newparam (`|GetArrayItem` (`/Game/TeamContent/BP/Player/InGame/Player/BP_CharactorData.ActionValue` (`/Game/TeamContent/BP/Player/InGame/Player/BP_Player.charaParam` _asbp_human))))
        (if (`KismetMathLibrary.InRange_FloatFloat` (`KismetMathLibrary.VSize` (- (`self.K2_GetActorLocation` _asbp_human) (`self.K2_GetActorLocation`))) 0.0 (`/Game/TeamContent/BP/Player/InGame/Player/BP_CharactorData.AttackRange` (`self.charaParam`)))
          (set `local.IsCanHitPlayer` true)
          (break)))))
  (if (`local.IsCanHitPlayer`)
    (bind _skillvalue (message `/Game/TeamContent/BP/Player/InGame/Ghost/BPI_GhostInterface.IGetSkillValue` (`GameplayStatics.GetGameState`)))
    (if (>= _skillvalue _output)
      (`self.RoS_SetGhostSkillValue` (- _skillvalue _output))
      (set `self.NowAtkDelay` (`/Game/TeamContent/BP/Player/InGame/Player/BP_CharactorData.AttackDelayTime` (`self.charaParam`)))
      (for _array_element (`local.LocalHuman`)
        (if (`KismetMathLibrary.InRange_FloatFloat` (`KismetMathLibrary.VSize` (- (`self.K2_GetActorLocation` _array_element) (`self.K2_GetActorLocation`))) 0.0 (`self.ATKRange`))
          (if (< (`KismetMathLibrary.Abs` (- (.yaw (`KismetMathLibrary.FindLookAtRotation` (`self.K2_GetActorLocation`) (`self.K2_GetActorLocation` _array_element))) (.yaw (`self.K2_GetActorRotation`)))) (`self.ATKAngle`))
            (bind _newparam_2 (message `/Game/TeamContent/BP/Player/InGame/Human/BPI_HumanFaerGaugeInterface.GetFaerValue` (`GameplayStatics.GetGameState`)))
            (if (>= _newparam_2 (`|GetArrayItem` (`/Game/TeamContent/BP/Player/InGame/Player/BP_CharactorData.ActionValue` (`/Game/TeamContent/BP/Player/InGame/Player/BP_Player.charaParam` _array_element))))
              (if (`/Game/TeamContent/BP/Player/InGame/Human/BP_Human.IsAlive` _array_element)
                (`self.RoS_AddDamageToPlayer` _array_element)
                (`KismetArrayLibrary.Array_Add` (`self.HitHumans`) _array_element)
                (`self.RoS_AddHitHumanIndex` (`/Game/TeamContent/BP/Player/InGame/Player/BP_Player.Index` _array_element))
                (`self.E_AddScore` 1)
                (set `local.IsHitPlayer` true))))))
      (if (`local.IsHitPlayer`)
        (`self.RoS_SetIsDragState` true)
        (`self.RoS_ChangeCollisionObjectType`)
        (return true)
        (else
          (`NiagaraFunctionLibrary.SpawnSystemAtLocation` "/Game/TeamContent/Graphic/Particle/NPS_OBAttack.NPS_OBAttack" (`self.K2_GetActorLocation`))
          (return true)))
      (else
        _)))
  (return false))

(fn `GetChangeGhost`
  (params (NewParam :type "Key Structure"))
  (returns (NewParam1 :type "/Game/TeamContent/BP/Player/InGame/Ghost/BP_Ghost Object Reference") (NewParam2 :type Boolean))
  (return null false))

(fn `GetGhostCharaParam`
  (returns (CharacterData :type "/Game/TeamContent/BP/Player/InGame/Player/BP_CharactorData Object Reference"))
  (return null))

(fn `GetGhostManager`
  (returns (NewParam :type "/Game/TeamContent/BP/Player/InGame/Manager/BP_GhostManager Object Reference"))
  (return null))

(fn `GetGhostSkillGaugeRate`
  (returns (NewParam :type "Float (double-precision)"))
  (return 0.0))

(fn `GetReallyGhostTransform`
  (params (self2 :type "Actor Object Reference"))
  (returns (ReturnValue :type "Vector Structure") (ReturnValue2 :type "Rotator Structure"))
  (return (`KismetMathLibrary.VLerp` (`self.K2_GetActorLocation` self2) (+ (`self.K2_GetActorLocation`) (* (* (`self.GetActorForwardVector`) -1.0) 40.0)) 0.1) (`KismetMathLibrary.RLerp` (`self.K2_GetActorRotation` self2) (`self.K2_GetActorRotation`) 0.1)))

(fn `GetScore`
  (returns (point :type Integer))
  (bind _score (message `/Game/TeamContent/BP/Player/InGame/Player/BPI_ToPlayerState.IGetPlayerScore` (`Controller.PlayerState` (`GameplayStatics.GetPlayerController` 0))))
  (return _score))

(fn `IGetGhostIndex`
  (returns (ghostIndex :type Integer))
  (return (`self.GhostIndex`)))

(fn `IGetIsCanChange`
  (returns (NewParam :type Boolean))
  (return false))

(fn `IGetPlayerGhost`
  (returns (ghost :type "/Game/TeamContent/BP/Player/InGame/Ghost/BP_Ghost Object Reference"))
  (return null))

(fn `IGetSkillValue`
  (returns (skillValue :type "Float (double-precision)"))
  (return 0.0))

(fn `SetOrnaments`
  (bind _sm_bag (`self.SM_Bag`))
  (bind _sm_ribbon (`self.SM_Ribbon`))
  (bind _sm_ribbon_2 (`self.SM_Ribbon`))
  (bind _sm_ribbon_3 (`self.SM_Ribbon`))
  (bind _sm_ribbon_4 (`self.SM_Ribbon`))
  (bind _sm_ribbon_5 (`self.SM_Ribbon`))
  (bind _sm_ribbon_6 (`self.SM_Ribbon`))
  (switch `int` (`KismetMathLibrary.RandomInteger` 6)
    (:`0`
      (`SceneComponent.SetVisibility` (`self.SM_Ribbon`) false false :!label _label)
      (`SceneComponent.SetVisibility` (`self.SM_Bag`) false false))
    (:`1`
      (goto _label))
    (:`2`
      (switch `int` (`KismetMathLibrary.RandomInteger` 4) :!label _label_2
        (:`0`
          (`SceneComponent.K2_AttachToComponent` _sm_ribbon_5 (`self.Mesh`) "Neck" "KeepRelative" "KeepRelative" "KeepRelative" true :!label _label_3)
          (`SceneComponent.K2_SetRelativeTransform` _sm_ribbon_5 (`KismetMathLibrary.MakeTransform` (0.0 0.0 10.0) (struct :`Roll` -90.0) (1.2 1.2 1.2)) false false))
        (:`1`
          (goto _label_3))
        (:`2`
          (`SceneComponent.K2_AttachToComponent` _sm_ribbon_2 (`self.Mesh`) "Neck" "KeepRelative" "KeepRelative" "KeepRelative" true)
          (`SceneComponent.K2_SetRelativeTransform` _sm_ribbon_2 (`KismetMathLibrary.MakeTransform` (18.0 -28.0 3.0) (struct :`Yaw` 30.0 :`Roll` -90.0) (0.7 0.7 0.7)) false false))
        (:`3`
          (`SceneComponent.K2_AttachToComponent` _sm_ribbon_3 (`self.Mesh`) "Neck" "KeepRelative" "KeepRelative" "KeepRelative" true)
          (`SceneComponent.K2_SetRelativeTransform` _sm_ribbon_3 (`KismetMathLibrary.MakeTransform` (-18.0 -28.0 3.0) (struct :`Yaw` -30.0 :`Roll` -90.0) (0.7 0.7 0.7)) false false)))
      (`SceneComponent.SetVisibility` (`self.SM_Bag`) false false))
    (:`3`
      (goto _label_2))
    (:`4`
      (`SceneComponent.K2_AttachToComponent` _sm_bag (`self.Mesh`) "Cest" "KeepRelative" "KeepRelative" "KeepRelative" true :!label _label_4)
      (`SceneComponent.K2_SetRelativeTransform` _sm_bag (`KismetMathLibrary.MakeTransform` (0.0 0.0 -8.0) (struct :`Roll` -90.0)) false false)
      (switch `int` (`KismetMathLibrary.RandomInteger` 8)
        (:`0`
          (`SceneComponent.SetVisibility` (`self.SM_Ribbon`) false false :!label _label_5))
        (:`1`
          (goto _label_5))
        (:`2`
          (goto _label_5))
        (:`3`
          (goto _label_5))
        (:`4`
          (`SceneComponent.K2_AttachToComponent` _sm_ribbon_4 (`self.Mesh`) "Neck" "KeepRelative" "KeepRelative" "KeepRelative" true :!label _label_6)
          (`SceneComponent.K2_SetRelativeTransform` _sm_ribbon_4 (`KismetMathLibrary.MakeTransform` (0.0 0.0 10.0) (struct :`Roll` -90.0) (1.2 1.2 1.2)) false false))
        (:`5`
          (goto _label_6))
        (:`6`
          (`SceneComponent.K2_AttachToComponent` _sm_ribbon_6 (`self.Mesh`) "Neck" "KeepRelative" "KeepRelative" "KeepRelative" true)
          (`SceneComponent.K2_SetRelativeTransform` _sm_ribbon_6 (`KismetMathLibrary.MakeTransform` (18.0 -28.0 3.0) (struct :`Yaw` 30.0 :`Roll` -90.0) (0.7 0.7 0.7)) false false))
        (:`7`
          (`SceneComponent.K2_AttachToComponent` _sm_ribbon (`self.Mesh`) "Neck" "KeepRelative" "KeepRelative" "KeepRelative" true)
          (`SceneComponent.K2_SetRelativeTransform` _sm_ribbon (`KismetMathLibrary.MakeTransform` (-18.0 -28.0 3.0) (struct :`Yaw` -30.0 :`Roll` -90.0) (0.7 0.7 0.7)) false false))))
    (:`5`
      (goto _label_4))))

(fn `TakeRandomIndex`
  (params (TakeNum :type Integer) (MinIndex :type Integer) (MaxIndex :type Integer) (NewParam :type "/Game/TeamContent/BP/Gimmick/BP_BlockFearAreaManager Object Reference"))
  (returns (RandomValues :type "Array of Integer"))
  (locals (TakedNum :type Integer) (Min :type Integer) (Max :type Integer) (TakedValue :type "Array of Integer") (random :type Integer :default 0) (LoopNum :type Integer))
  (set `local.Min` MinIndex)
  (set `local.Max` MaxIndex)
  (while (and (> TakeNum (`local.TakedNum`)) (< (`local.LoopNum`) 100))
    (`/Engine/EditorBlueprintResources/StandardMacros.IncrementInt` (`local.LoopNum`)
      (:`  `
        (set `local.random` (`KismetMathLibrary.RandomIntegerInRange` (`local.Min`) (`local.Max`)))
        (if (and (== (`KismetArrayLibrary.Array_Find` (`local.TakedValue`) (`local.random`)) -1) (`/Game/TeamContent/BP/Gimmick/BP_BlockFearAreaManager.GetIsActive` NewParam (`local.random`)))
          (`KismetArrayLibrary.Array_Add` (`local.TakedValue`) (`local.random`))
          (`/Engine/EditorBlueprintResources/StandardMacros.IncrementInt` (`local.TakedNum`))))))
  (return (`local.TakedValue`)))

(fn `UserConstructionScript`
  (`parent.UserConstructionScript`))