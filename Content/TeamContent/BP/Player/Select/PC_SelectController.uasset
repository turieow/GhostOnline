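; PC_SelectController is a player controller that puts up the title/login UI and frames the view on a tagged camera.
; On BeginPlay it creates WBP_Title, plays its fade animation, shows the mouse cursor and sets Game and UI input.
; BeginPlay and Possess both lead into a short delay, then set the view target to the first actor tagged MainCamera.
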(event `self.ReceiveBeginPlay`
  (bind _returnvalue (`GameplayStatics.GetPlayerController` 0))
  (`parent.ReceiveBeginPlay`)
  (`self.E_CreateLoginUI`)
  (set `PlayerController.bShowMouseCursor` true _returnvalue)
  (`WidgetBlueprintLibrary.SetInputMode_GameAndUIEx` _returnvalue null)
  (`KismetSystemLibrary.Delay` 3.0 :!label _label)
  (bind _outactors (`GameplayStatics.GetAllActorsWithTag` "MainCamera"))
  (`self.SetViewTargetWithBlend` (`GameplayStatics.GetPlayerController` 0) (`|GetArrayItem` _outactors) 0.0 "VTBlend_Linear" 0.0 false))

(event `self.ReceivePossess`
  (params (PossessedPawn :type "Pawn Object Reference"))
  (goto _label))

(event `E_CreateLoginUI`
  (bind _returnvalue (`|CreateWidget` "/Game/TeamContent/BP/UI/WBP_Title.WBP_Title_C" self))
  (bind _output_get (set `self.LoginUI` _returnvalue))
  (`/Engine/EditorBlueprintResources/StandardMacros.IsValid` _output_get
    (:`Is Valid`
      (`UserWidget.AddToViewport` _output_get 0)
      (message `/Game/TeamContent/BP/UI/BPI_ToUI.FadeAnimation` _output_get false 1.0))))

(fn `UserConstructionScript`)