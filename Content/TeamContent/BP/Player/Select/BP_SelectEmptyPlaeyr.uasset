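; Character Blueprint for a player select context that gives each of four players a distinct cloth material and handles basic movement input.
; BeginPlay sets mesh material slot 1 from the player ID, while a RoS event forwards material changes to an MC event, suggesting server-to-multicast replication.
; MoveForward and MoveRight build their direction using the camera forward vector's Z component as yaw, rather than camera rotation.
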(event `self.ReceiveBeginPlay`
  (`self.E_SetPlayerMaterial` (`self.ID`)))

(event `InputAxis|MoveForward` :consume false :overrideparent false
  (params (AxisValue :type "Float (single-precision)"))
  (bind (_returnvalue_x _returnvalue_y _returnvalue_z) (`KismetMathLibrary.BreakVector` (`self.GetActorForwardVector` (`GameplayStatics.GetPlayerCameraManager` 0))))
  ;[1 1 1] movementinput
  (`self.AddMovementInput` (`KismetMathLibrary.GetForwardVector` (`KismetMathLibrary.MakeRotator` 0.0 0.0 _returnvalue_z)) AxisValue))

(event `InputAxis|MoveRight` :overrideparent false
  (params (AxisValue :type "Float (single-precision)"))
  (bind (_returnvalue_x _returnvalue_y _returnvalue_z) (`KismetMathLibrary.BreakVector` (`self.GetActorForwardVector` (`GameplayStatics.GetPlayerCameraManager` 0))))
  ;[1 1 1] movementinput
  (`self.AddMovementInput` (`KismetMathLibrary.GetRightVector` (`KismetMathLibrary.MakeRotator` 0.0 0.0 _returnvalue_z)) AxisValue))

(event `RoS_SetPlayerMaterial`
  (params (Index :type Integer))
  (`self.MC_SetPlayerMaterial` Index))

(event `MC_SetPlayerMaterial`
  (params (Index :type Integer))
  ;[1 1 1] マテリアル設定
  (`PrimitiveComponent.SetMaterial` (`self.Mesh`) 1 (select `int` Index :`0` "/Game/TeamContent/Graphic/Mesh/Character/Cloth1P.Cloth1P" :`1` "/Game/TeamContent/Graphic/Mesh/Character/Cloth2P.Cloth2P" :`2` "/Game/TeamContent/Graphic/Mesh/Character/Cloth3P.Cloth3P" :`3` "/Game/TeamContent/Graphic/Mesh/Character/Cloth4P.Cloth4P" :!type "MaterialInterface Object Reference")))

(event `E_SetPlayerMaterial`
  (params (Index :type Integer))
  (`PrimitiveComponent.SetMaterial` (`self.Mesh`) 1 (select `int` Index :`0` "/Game/TeamContent/Graphic/Mesh/Character/Cloth1P.Cloth1P" :`1` "/Game/TeamContent/Graphic/Mesh/Character/Cloth2P.Cloth2P" :`2` "/Game/TeamContent/Graphic/Mesh/Character/Cloth3P.Cloth3P" :`3` "/Game/TeamContent/Graphic/Mesh/Character/Cloth4P.Cloth4P" :!type "MaterialInterface Object Reference")))

(fn `UserConstructionScript`)