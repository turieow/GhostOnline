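; BP_BigDoll is a crowned NPC doll that wakes on the game state's time-up flag to attack humans.
; Tick uses DoOnce gates to start or stop its AI brain logic, triggering a target camera and gathering BP_Human actors on waking.
; While awake, contact knocks back ghosts and downed humans.
; ATK box-traces forward, damaging humans via RoS_AddDamageToHuman, dropping them from its list and launching them.
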(event `self.ReceiveBeginPlay`
  (`self.SetCrown`))

(event `self.ReceiveTick`
  (params (DeltaSeconds :type "Float (single-precision)"))
  (bind _returnvalue (`AIBlueprintHelperLibrary.GetAIController` (`self.GetController`)))
  (bind _braincomponent (`AIController.BrainComponent` _returnvalue))
  (bind _istimeup (message `/Game/TeamContent/BP/System/MainGame/BPI_ToGameState.IGetTimeUpFlag` (`GameplayStatics.GetGameState`)))
  (bind _output_get (set `self.IsGetUp` _istimeup))
  (`/Engine/EditorBlueprintResources/StandardMacros.IsValid` _returnvalue
    (:`Is Valid`
      (if _output_get
        (`/Engine/EditorBlueprintResources/StandardMacros.DoOnce` false :!label _label
          (:`Completed`
            (`BrainComponent.StartLogic` _braincomponent)
            (message `/Game/TeamContent/BP/System/MainGame/BPI_ToGameState.IStartTargetCamera` (`GameplayStatics.GetGameState`) self 50.0)
            (bind _outactors (`GameplayStatics.GetAllActorsOfClass` "/Game/TeamContent/BP/Player/InGame/Human/BP_Human.BP_Human_C"))
            (bind _output_get_2 (set `self.Humans` _outactors))
            (if (!= (`KismetArrayLibrary.Array_Length` _output_get_2) 0)
              (for (_array_element _array_index) _output_get_2
                (if (not (`/Game/TeamContent/BP/Player/InGame/Human/BP_Human.IsAlive` _array_element))
                  (`KismetArrayLibrary.Array_Remove` _output_get_2 _array_index)))
              (goto _label_2 :!via `Reset`)
              (else
                (goto _label_2 :!via `Reset`)))))
        (else
          (`/Engine/EditorBlueprintResources/StandardMacros.DoOnce` false :!label _label_2
            (:`Completed`
              (`BrainComponent.StopLogic` _braincomponent "")
              (goto _label :!via `Reset`))))))))

(event `self.Sphere.OnComponentBeginOverlap`
  (params (OverlappedComponent :type "PrimitiveComponent Object Reference") (OtherActor :type "Actor Object Reference") (OtherComp :type "PrimitiveComponent Object Reference") (OtherBodyIndex :type Integer) (bFromSweep :type Boolean) (SweepResult :type "HitResult Structure (by ref)"))
  (`self.KnockBack` OtherActor))

(event `self.Mesh.OnComponentHit`
  (params (HitComponent :type "PrimitiveComponent Object Reference") (OtherActor :type "Actor Object Reference") (OtherComp :type "PrimitiveComponent Object Reference") (NormalImpulse :type "Vector Structure") (Hit :type "HitResult Structure (by ref)"))
  (`self.KnockBack` OtherActor))

(event `self.CapsuleComponent.OnComponentHit`
  (params (HitComponent :type "PrimitiveComponent Object Reference") (OtherActor :type "Actor Object Reference") (OtherComp :type "PrimitiveComponent Object Reference") (NormalImpulse :type "Vector Structure") (Hit :type "HitResult Structure (by ref)"))
  (`self.KnockBack` OtherActor))

(event `KnockBack`
  (params (NewParam :type "Actor Object Reference"))
  (if (`self.IsGetUp`)
    (bind _asbp_ghost (cast `/Game/TeamContent/BP/Player/InGame/Ghost/BP_Ghost` NewParam)
      (:`then`
        (bind (_returnvalue_x _returnvalue_y) (`KismetMathLibrary.BreakVector` (- (`self.K2_GetActorLocation` _asbp_ghost) (`self.K2_GetActorLocation`))))
        (`self.LaunchCharacter` _asbp_ghost (+ (* (`KismetMathLibrary.Normal` (`KismetMathLibrary.MakeVector` _returnvalue_x _returnvalue_y)) 500.0) (0.0 0.0 500.0)) false false))
      (:`CastFailed`
        (bind _asbp_human (cast `/Game/TeamContent/BP/Player/InGame/Human/BP_Human` NewParam))
        (if (`/Game/TeamContent/BP/Player/InGame/Human/BP_Human.IsDownOver` _asbp_human)
          (bind (_returnvalue_x_2 _returnvalue_y_2) (`KismetMathLibrary.BreakVector` (- (`self.K2_GetActorLocation` _asbp_human) (`self.K2_GetActorLocation`))))
          (`self.LaunchCharacter` _asbp_human (+ (* (`KismetMathLibrary.Normal` (`KismetMathLibrary.MakeVector` _returnvalue_x_2 _returnvalue_y_2)) 100.0) (0.0 0.0 100.0)) false false))))))

(event `RoS_AddDamageToHuman`
  (params (Human :type "Object Object Reference"))
  (message `/Game/TeamContent/BP/Player/InGame/Human/BPI_HumanInterface.AddHumanDamage` Human (`self.K2_GetActorLocation`)))

(fn `ATK`
  (bind _returnvalue (`SceneComponent.K2_GetComponentLocation` (`self.Arrow1`)))
  (bind _outhits (`KismetSystemLibrary.BoxTraceMulti` :`Start` _returnvalue :`End` (+ _returnvalue (* (`SceneComponent.GetForwardVector` (`self.CapsuleComponent`)) 100.0)) :`HalfSize` (50.0 50.0 0.5) :`Orientation` (`self.K2_GetActorRotation`) :`TraceChannel` "TraceTypeQuery1" :`DrawDebugType` "ForDuration"))
  (for _array_element _outhits
    (bind _asbp_human (cast `/Game/TeamContent/BP/Player/InGame/Human/BP_Human` (`.HitActor` (`GameplayStatics.BreakHitResult` _array_element))))
    (`self.RoS_AddDamageToHuman` _asbp_human)
    (`self.DiedHuman` _asbp_human)
    (bind (_returnvalue_x _returnvalue_y) (`KismetMathLibrary.BreakVector` (- (`self.K2_GetActorLocation` _asbp_human) (`self.K2_GetActorLocation`))))
    (`self.LaunchCharacter` _asbp_human (+ (* (`KismetMathLibrary.Normal` (`KismetMathLibrary.MakeVector` _returnvalue_x _returnvalue_y)) 100.0) (0.0 0.0 300.0)) false false)
    (set `self.IsAttackFlag` false)))

(fn `DiedHuman`
  (params (NewParam :type "/Game/TeamContent/BP/Player/InGame/Human/BP_Human Object Reference"))
  (bind _humans (`self.Humans`))
  (`KismetArrayLibrary.Array_Remove` _humans (`KismetArrayLibrary.Array_Find` _humans NewParam)))

(fn `SetCrown`
  (bind _sm_crown (`self.SM_Crown`))
  (`SceneComponent.K2_AttachToComponent` _sm_crown (`self.Mesh`) "Neck" "KeepRelative" "KeepRelative" "KeepRelative" true)
  (`SceneComponent.K2_SetRelativeTransform` _sm_crown (`KismetMathLibrary.MakeTransform` (0.0 -25.0 0.0) (struct :`Roll` -90.0) (0.2 0.2 0.2)) false false))

(fn `UserConstructionScript`)