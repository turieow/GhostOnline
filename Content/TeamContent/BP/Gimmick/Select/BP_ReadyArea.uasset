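; BP_ReadyArea is a ready-up trigger area that marks the local player as ready for matching and shows how many players are ready out of four.
; Box overlaps by player pawn 0 switch the matching status on that player's PlayerState through an interface call.
; On BeginPlay and every Tick, it polls the GameState PlayerArray, counts ready statuses and rewrites the TextRender counter.
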(event `self.ReceiveBeginPlay`
  (`self.E_SetText`))

(event `self.ReceiveTick`
  (params (DeltaSeconds :type "Float (single-precision)"))
  (`self.E_SetText`))

(event `self.Box.OnComponentBeginOverlap`
  (params (OverlappedComponent :type "PrimitiveComponent Object Reference") (OtherActor :type "Actor Object Reference") (OtherComp :type "PrimitiveComponent Object Reference") (OtherBodyIndex :type Integer) (bFromSweep :type Boolean) (SweepResult :type "HitResult Structure (by ref)"))
  (if (== OtherActor (`GameplayStatics.GetPlayerPawn` 0))
    (message `/Game/TeamContent/BP/Player/InGame/Player/BPI_ToPlayerState.ISetMatchingStatus` (`Controller.PlayerState` (`GameplayStatics.GetPlayerController` 0)) "NewEnumerator2")))

(event `self.Box.OnComponentEndOverlap`
  (params (OverlappedComponent :type "PrimitiveComponent Object Reference") (OtherActor :type "Actor Object Reference") (OtherComp :type "PrimitiveComponent Object Reference") (OtherBodyIndex :type Integer))
  (if (== OtherActor (`GameplayStatics.GetPlayerPawn` 0))
    (message `/Game/TeamContent/BP/Player/InGame/Player/BPI_ToPlayerState.ISetMatchingStatus` (`Controller.PlayerState` (`GameplayStatics.GetPlayerController` 0)) "NewEnumerator1")))

(event `E_SetText`
  ;[1 1 1] 参加状況をテキスト表示
  (`TextRenderComponent.K2_SetText` (`self.TextRender`) (`KismetTextLibrary.Conv_StringToText` (`KismetStringLibrary.Concat_StrStr` "READY " (`KismetStringLibrary.Conv_IntToString` (`self.GetAlreadyPlayerNum`)) "/4"))))

(fn `GetAlreadyPlayerNum`
  (returns (AlreadyNum :type Integer))
  (locals (num :type Integer))
  (for _array_element (`GameStateBase.PlayerArray` (`GameplayStatics.GetGameState`))
    (bind _isready (message `/Game/TeamContent/BP/Player/InGame/Player/BPI_ToPlayerState.IGetMatchingStatus` _array_element))
    (if (`|EnumEquality` _isready "NewEnumerator2")
      (`/Engine/EditorBlueprintResources/StandardMacros.IncrementInt` (`local.num`))))
  (return (`local.num`)))

(fn `UserConstructionScript`)