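; BP_RosaryEffectArea is a timed area effect that slows ghosts inside a sphere of configurable radius.
; Sphere overlap events send WalkSlowMessage on or off to actors tagged "Ghost" as they enter and leave.
; After EffectTime, it clears the slow on any overlapping BP_Ghost actors and destroys itself.
; An unconnected branch that would spawn zone Niagara effects at random navigable points never runs.
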(event `self.ReceiveBeginPlay`
  (`SphereComponent.SetSphereRadius` (`self.Sphere`) (`self.AreaRadius`) true)
  (`KismetSystemLibrary.Delay` (`self.EffectTime`))
  (bind (_outactors _returnvalue) (`KismetSystemLibrary.ComponentOverlapActors` null (`SceneComponent.K2_GetComponentToWorld` (`self.Sphere`)) (`|MakeArray` "ObjectTypeQuery1" "ObjectTypeQuery2" :!type "EObjectTypeQuery Enum") "/Game/TeamContent/BP/Player/InGame/Ghost/BP_Ghost.BP_Ghost_C"))
  (if _returnvalue
    (for _array_element _outactors
      (message `/Game/TeamContent/BP/Player/InGame/Ghost/BPI_GhostInterface.WalkSlow` _array_element false)))
  (`self.K2_DestroyActor`))

(event `self.Sphere.OnComponentBeginOverlap`
  (params (OverlappedComponent :type "PrimitiveComponent Object Reference") (OtherActor :type "Actor Object Reference") (OtherComp :type "PrimitiveComponent Object Reference") (OtherBodyIndex :type Integer) (bFromSweep :type Boolean) (SweepResult :type "HitResult Structure (by ref)"))
  (if (`self.ActorHasTag` OtherActor "Ghost")
    (message `/Game/TeamContent/BP/Player/InGame/Ghost/BPI_GhostInterface.WalkSlow` OtherActor true)))

(event `self.Sphere.OnComponentEndOverlap`
  (params (OverlappedComponent :type "PrimitiveComponent Object Reference") (OtherActor :type "Actor Object Reference") (OtherComp :type "PrimitiveComponent Object Reference") (OtherBodyIndex :type Integer))
  (if (`self.ActorHasTag` OtherActor "Ghost")
    (message `/Game/TeamContent/BP/Player/InGame/Ghost/BPI_GhostInterface.WalkSlow` OtherActor false)))

(event `self.ReceiveTick`
  (params (DeltaSeconds :type "Float (single-precision)")))

(fn `UserConstructionScript`)