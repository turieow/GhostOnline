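; Light gimmick actor that shows a mesh, likely a beam, aimed from its Cube at a linked TargetArea's Area.
; Each Tick rotates both meshes toward the area with a 90-degree pitch offset, stretching StaticMesh's length with distance and narrowing its width.
; StaticMesh is visible only while the area's light is on and its opacity exceeds a threshold.
; BeginPlay prints a warning when no TargetArea is set.
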(event `self.ReceiveBeginPlay`
  (`/Engine/EditorBlueprintResources/StandardMacros.IsValid` (`self.TargetArea`)
    (:`Is Not Valid`
      (`KismetSystemLibrary.PrintString` "LightGimmick--BP_Light::NoneLightArea"))))

(event `self.ReceiveTick`
  (params (DeltaSeconds :type "Float (single-precision)"))
  (bind _targetarea (`self.TargetArea`))
  (bind _returnvalue (`SceneComponent.K2_GetComponentLocation` (`self.Cube`)))
  (bind _returnvalue_2 (`SceneComponent.K2_GetComponentLocation` (`/Game/TeamContent/BP/Gimmick/BP_LightArea.Area` _targetarea)))
  (bind (_returnvalue_roll _returnvalue_pitch _returnvalue_yaw) (`KismetMathLibrary.BreakRotator` (`KismetMathLibrary.FindLookAtRotation` _returnvalue _returnvalue_2)))
  (bind _returnvalue_3 (`KismetMathLibrary.VSize` (- _returnvalue _returnvalue_2)))
  (bind _returnvalue_4 (* (- 6000.0 _returnvalue_3) (* 0.0001 (`self.UpRadiusValue`))))
  (`/Engine/EditorBlueprintResources/StandardMacros.IsValid` _targetarea
    (:`Is Valid`
      (`|ExecutionSequence`
        (:`then_0`
          (if (`/Game/TeamContent/BP/Gimmick/BP_LightArea.IsLightOnState` _targetarea)
            (`SceneComponent.SetVisibility` (`self.StaticMesh`) (> (`/Game/TeamContent/BP/Gimmick/BP_LightArea.LightOpacity` _targetarea) 0.6) false)
            (`SceneComponent.K2_SetWorldRotation` (`self.Cube`) (`KismetMathLibrary.MakeRotator` _returnvalue_roll (+ _returnvalue_pitch 90.0) _returnvalue_yaw) false false)
            (`SceneComponent.K2_SetWorldRotation` (`self.StaticMesh`) (`KismetMathLibrary.MakeRotator` _returnvalue_roll (+ _returnvalue_pitch 90.0) _returnvalue_yaw) false false)
            (`SceneComponent.SetWorldScale3D` (`self.StaticMesh`) (`KismetMathLibrary.MakeVector` _returnvalue_4 _returnvalue_4 (* _returnvalue_3 (* 0.001 (`self.DownScaleValue`)))))
            (else
              (`SceneComponent.SetVisibility` (`self.StaticMesh`) false false))))))))

(fn `UserConstructionScript`)