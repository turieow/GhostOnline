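; Light area gimmick that periodically switches on a roaming decal light and notifies Ghost-tagged actors entering or leaving its sphere.
; Tick cycles lifetime and delay from DA_Gimmick parameters, moving the area between random MoveLoc offsets while lit.
; Timelines drive dynamic-material opacity for switching on and off, hiding the decal at low values to flicker or fade.
; It also binds to BP_GhostManager possession events and can re-notify ghosts already inside the light.
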(event `self.ReceiveBeginPlay`
  (bind _decal (`self.Decal`))
  (`self.E_BindGhostChange`)
  (`/Engine/EditorBlueprintResources/StandardMacros.IsValid` (`self.DynamicMaterial`)
    (:`Is Valid`
      _)
    (:`Is Not Valid`
      (bind _returnvalue (`KismetMaterialLibrary.CreateDynamicMaterialInstance` (`DecalComponent.DecalMaterial` _decal)))
      (set `self.DynamicMaterial` _returnvalue)))
  (`DecalComponent.SetDecalMaterial` _decal (`self.DynamicMaterial`))
  (bind _output_get (set `self.GimmickParam` "/Game/TeamContent/DataAsset/DA_Gimmick.DA_Gimmick"))
  (`SphereComponent.SetSphereRadius` (`self.Area`) (`/Game/TeamContent/BP/Gimmick/BP_GimmickData.SL_AreaRadius` _output_get) true)
  (`SceneComponent.SetRelativeScale3D` (`self.Decal`) (`/Game/TeamContent/BP/Gimmick/BP_GimmickData.SL_DecalScale` _output_get)))

(event `self.ReceiveTick`
  (params (DeltaSeconds :type "Float (single-precision)"))
  (bind _gimmickparam (`self.GimmickParam`))
  (bind _decal (`self.Decal`))
  (`|ExecutionSequence`
    (:`then_0`
      (`/Engine/EditorBlueprintResources/StandardMacros.DoOnce` false :!label _label
        (:`Completed`
          (`self.ActionGimmick`)
          (`KismetSystemLibrary.Delay` (`/Game/TeamContent/BP/Gimmick/BP_GimmickData.SL_LifeTime` _gimmickparam))
          (`KismetSystemLibrary.Delay` (`/Game/TeamContent/BP/Gimmick/BP_GimmickData.SL_Delay` _gimmickparam))
          (goto _label :!via `Reset`))))
    (:`then_1`
      (`self.LifeTimeTick`)
      (if (`self.IsLighting`)
        (`self.ChangeMoveTarget`)
        (`self.Move`)
        (`SceneComponent.SetVisibility` _decal true false)
        (if (not (> (`self.NowLifeTime`) 1.0))
          (`self.RevasaeLight`))
        (else
          (`SceneComponent.SetVisibility` _decal false false))))))

(event `RevasaeLight`
  (bind _decal (`self.Decal`))
  (`/Engine/EditorBlueprintResources/StandardMacros.DoOnce` false :!label _label_2
    (:`Completed`
      (bind (_direction `_新規track_0`) (`Timeline|Lightoff` :!label _label_3)
        (:`Update`
          (set `self.LightOpacity` `_新規track_0`)
          (bind _returnvalue (> `_新規track_0` 0.65))
          (if _returnvalue
            (`SceneComponent.SetVisibility` _decal _returnvalue false)
            (`MaterialInstanceDynamic.SetScalarParameterValue` (`self.DynamicMaterial`) "Opacity" `_新規track_0`)
            (else
              (`SceneComponent.SetVisibility` _decal false false))))
        (:`Finished`
          (`MaterialInstanceDynamic.SetScalarParameterValue` (`self.DynamicMaterial`) "Opacity" 1.0)
          (set `self.IsLightOnState` false)
          (`PrimitiveComponent.SetCollisionEnabled` (`self.Area`) "NoCollision"))))))

(event `LifeTimeTick`
  (set `self.NowLifeTime` (- (`self.NowLifeTime`) (`GameplayStatics.GetWorldDeltaSeconds`)))
  (if (> (`self.NowLifeTime`) 0.0)
    (set `self.IsLighting` true)
    (goto _label_4 :!via `Reset`)
    (else
      (set `self.IsLighting` false)
      (`/Engine/EditorBlueprintResources/StandardMacros.DoOnce` true :!label _label_4
        (:`Completed`
          (`self.ResetLight`)
          (`self.ResetRevaseLight`))))))

(event `ResetRevaseLight`
  (`|ExecutionSequence`
    (:`then_0`
      (goto _label_2 :!via `Reset`))
    (:`then_1`
      (goto _label_3 :!via `SetNewTime`))))

(event `self.ActionGimmick`
  (bind _moveloc (`self.MoveLoc`))
  (bind _decal (`self.Decal`))
  (if (not (`self.IsLighting`))
    (`/Engine/EditorBlueprintResources/StandardMacros.DoOnce` false :!label _label_5
      (:`Completed`
        (set `self.IsLightOnState` true)
        (bind _output_get (set `self.EndLoc` (+ (`self.K2_GetActorLocation`) (`|GetArrayItem` _moveloc (`KismetMathLibrary.RandomIntegerInRange` 0 (`KismetArrayLibrary.Array_LastIndex` _moveloc))))))
        (`SceneComponent.K2_SetWorldLocation` (`self.Area`) _output_get false false)
        (set `self.IsChangeMoveTarget` true)
        (`PrimitiveComponent.SetCollisionEnabled` (`self.Area`) "QueryAndPhysics")
        (bind (_direction _opacity) (`Timeline|Light` :!label _label_6)
          (:`Update`
            (set `self.LightOpacity` _opacity)
            (bind _returnvalue (> _opacity 0.65))
            (if _returnvalue
              (`SceneComponent.SetVisibility` _decal _returnvalue false)
              (`MaterialInstanceDynamic.SetScalarParameterValue` (`self.DynamicMaterial`) "Opacity" (`self.LightOpacity`))
              (else
                (`SceneComponent.SetVisibility` _decal false false))))
          (:`Finished`
            (set `self.NowLifeTime` (`/Game/TeamContent/BP/Gimmick/BP_GimmickData.SL_LifeTime` (`self.GimmickParam`)))
            (`MaterialInstanceDynamic.SetScalarParameterValue` (`self.DynamicMaterial`) "Opacity" 1.0)))))))

(event `ResetLight`
  (`|ExecutionSequence`
    (:`then_0`
      (goto _label_5 :!via `Reset`))
    (:`then_1`
      (goto _label_6 :!via `SetNewTime`))))

(event `self.Area.OnComponentBeginOverlap`
  (params (OverlappedComponent :type "PrimitiveComponent Object Reference") (OtherActor :type "Actor Object Reference") (OtherComp :type "PrimitiveComponent Object Reference") (OtherBodyIndex :type Integer) (bFromSweep :type Boolean) (SweepResult :type "HitResult Structure (by ref)"))
  (if (`self.ActorHasTag` OtherActor "Ghost")
    (message `/Game/TeamContent/BP/Player/InGame/Ghost/BPI_GhostInterface.InLight` OtherActor)))

(event `self.Area.OnComponentEndOverlap`
  (params (OverlappedComponent :type "PrimitiveComponent Object Reference") (OtherActor :type "Actor Object Reference") (OtherComp :type "PrimitiveComponent Object Reference") (OtherBodyIndex :type Integer))
  (if (`self.ActorHasTag` OtherActor "Ghost")
    (message `/Game/TeamContent/BP/Player/InGame/Ghost/BPI_GhostInterface.OutLight` OtherActor)))

(event `E_CheckGhost`
  (if (`self.IsLightOnState`)
    (bind (_outactors _returnvalue) (`KismetSystemLibrary.SphereOverlapActors` (`self.K2_GetActorLocation`) 3000.0 (`|MakeArray` "ObjectTypeQuery3" :!type "EObjectTypeQuery Enum")))
    (if _returnvalue
      (for _array_element _outactors
        (if (`PrimitiveComponent.IsOverlappingActor` (`self.Area`) _array_element)
          (if (`self.ActorHasTag` _array_element "Ghost")
            (message `/Game/TeamContent/BP/Player/InGame/Ghost/BPI_GhostInterface.InLight` _array_element)))))))

(event `E_BindGhostChange`
  (bind _returnvalue (`GameplayStatics.GetActorOfClass` "/Game/TeamContent/BP/Player/InGame/Manager/BP_GhostManager.BP_GhostManager_C"))
  (`/Engine/EditorBlueprintResources/StandardMacros.IsValid` _returnvalue
    (:`Is Valid`
      (add `/Game/TeamContent/BP/Player/InGame/Manager/BP_GhostManager.OnPossesed` _returnvalue (`|CreateDelegate` :!event `E_CheckGhost`)))))

(fn `ChangeMoveTarget`
  (bind _moveloc (`self.MoveLoc`))
  (bind _returnvalue (`KismetArrayLibrary.Array_LastIndex` _moveloc))
  (bind _returnvalue_2 (+ (`|GetArrayItem` _moveloc) (`self.K2_GetActorLocation`)))
  (if (`KismetArrayLibrary.Array_IsValidIndex` _moveloc)
    (if (`self.IsChangeMoveTarget`)
      (if (> _returnvalue 0)
        (set `self.StartLoc` (`self.EndLoc`))
        (set `self.EndLoc` (+ (`self.K2_GetActorLocation`) (`|GetArrayItem` _moveloc (`KismetMathLibrary.RandomIntegerInRange` 0 _returnvalue))))
        (else
          (set `self.StartLoc` _returnvalue_2)
          (set `self.EndLoc` _returnvalue_2)))
      (set `self.IsChangeMoveTarget` false))
    (else
      (`KismetSystemLibrary.PrintString` "NoneLightLoc"))))

(fn `IsCanPlay`
  (params (Player :type "Actor Object Reference"))
  (returns (playing :type Boolean))
  (return false))

(fn `Move`
  (if (> (`KismetMathLibrary.VSize` (- (`self.EndLoc`) (`SceneComponent.K2_GetComponentLocation` (`self.Area`)))) (/ (`/Game/TeamContent/BP/Gimmick/BP_GimmickData.SL_Speed` (`self.GimmickParam`)) 10.0))
    (`SceneComponent.K2_AddWorldOffset` (`self.Area`) (* (`KismetMathLibrary.Normal` (- (`self.EndLoc`) (`self.StartLoc`)) 1.0) (* (`/Game/TeamContent/BP/Gimmick/BP_GimmickData.SL_Speed` (`self.GimmickParam`)) (`GameplayStatics.GetWorldDeltaSeconds`))) false false)
    (else
      (`SceneComponent.K2_SetWorldLocation` (`self.Area`) (`self.EndLoc`) false false)
      (set `self.IsChangeMoveTarget` true))))

(fn `UserConstructionScript`)