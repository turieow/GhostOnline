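; BP_BlockFearArea is a table-lamp gimmick representing a switchable fear-blocking area, with a debug draw of its radius.
; Enabling or disabling it plays separate flicker timelines, thresholded by a macro that fires only on state changes.
; These drive point and spot light visibility and the lamp's dynamic-material emissive.
; A widget appears once the lamp finishes switching off and rotates every tick to face the player camera.
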(event `self.ReceiveBeginPlay`
  (bind _pointlight (`self.PointLight`))
  (bind _active (`self.Active`))
  (`parent.ReceiveBeginPlay`)
  (`ActorComponent.SetActive` _pointlight _active false)
  (`SceneComponent.SetVisibility` _pointlight _active false)
  (set `self.NowLightOn` _active)
  (`SceneComponent.SetVisibility` (`self.Widget`) false false)
  (`self.LightOn/Off` _active))

(event `/Game/TeamContent/BP/Gimmick/BPI_Gimick.SetBlockFearAreaEnable`
  (params (enable :type Boolean))
  (if enable
    (if (not (`self.NowLightOn`))
      (`|ExecutionSequence`
        (:`then_0`
          (bind (_direction `_新規track_0`) (`Timeline|タイムライン_1` :!via `Stop` :!label _label)
            (:`Update`
              (bind _visible (`self.TenmetuVisibility` `_新規track_0`)
                (:`Different`
                  (bind _output_get (set `self.Active` _visible))
                  (`SceneComponent.ToggleVisibility` (`self.PointLight`) _output_get)
                  (`SceneComponent.ToggleVisibility` (`self.SpotLight1`) _output_get)
                  (`self.LightOn/Off` _output_get)
                  (set `self.NowLightOn` false))))
            (:`Finished`
              (bind _output_get_2 (set `self.Active` enable :!label _label_2))
              (`SceneComponent.ToggleVisibility` (`self.PointLight`) _output_get_2)
              (`SceneComponent.ToggleVisibility` (`self.SpotLight1`) _output_get_2)
              (`self.LightOn/Off` _output_get_2)
              (if (not _output_get_2)
                (`SceneComponent.SetVisibility` (`self.Widget`) true false)))))
        (:`then_1`
          (bind (_direction_2 `_新規track_0_2`) (`Timeline|タイムライン_0` :!via `PlayFromStart` :!label _label_3)
            (:`Update`
              (bind _visible_2 (`self.TenmetuVisibility` `_新規track_0_2`)
                (:`Different`
                  (bind _output_get_3 (set `self.Active` _visible_2))
                  (`SceneComponent.ToggleVisibility` (`self.PointLight`) _output_get_3)
                  (`SceneComponent.ToggleVisibility` (`self.SpotLight1`) _output_get_3)
                  (`self.LightOn/Off` _output_get_3)
                  (`SceneComponent.SetVisibility` (`self.Widget`) false false)
                  (set `self.NowLightOn` true))))
            (:`Finished`
              (goto _label_2))))))
    (elif (`self.NowLightOn`)
      (`|ExecutionSequence`
        (:`then_0`
          (goto _label_3 :!via `Stop`))
        (:`then_1`
          (goto _label :!via `PlayFromStart`))))))

(event `E_DrawRadius`
  (`KismetSystemLibrary.DrawDebugSphere` (`self.K2_GetActorLocation`) (`/Game/TeamContent/BP/Gimmick/BP_GimmickData.BF_AreaRadius` (`self.GimmickParam`)) 12 (struct :`G` 0.061501 :`B` 1.0 :`A` 1.0) 3.0))

(event `self.ReceiveTick`
  (params (DeltaSeconds :type "Float (single-precision)"))
  (`|ExecutionSequence`
    (:`then_0`
      (`/Engine/EditorBlueprintResources/StandardMacros.IsValid` (`self.Widget`)
        (:`Is Valid`
          (`SceneComponent.K2_SetWorldRotation` (`self.Widget`) (`KismetMathLibrary.FindLookAtRotation` (`self.K2_GetActorLocation`) (`PlayerCameraManager.GetCameraLocation` (`GameplayStatics.GetPlayerCameraManager` 0))) false false))))))

(fn `GetChangeGhost`
  (params (NewParam :type "Key Structure"))
  (returns (NewParam1 :type "/Game/TeamContent/BP/Player/InGame/Ghost/BP_Ghost Object Reference") (NewParam2 :type Boolean))
  (return null false))

(fn `GetGhostFaerGaugeRate`
  (returns (NewParam :type "Float (double-precision)"))
  (return 0.0))

(fn `GetGhostManager`
  (returns (NewParam :type "/Game/TeamContent/BP/Player/InGame/Manager/BP_GhostManager Object Reference"))
  (return null))

(fn `GettenmetuVisibitliy`
  (params (A :type "Float (double-precision)"))
  (returns (ReturnValue :type Boolean))
  (bind _returnvalue (> A 0.5))
  (if (!= _returnvalue (`self.Active`))
    (return _returnvalue)))

(fn `LightOn/Off`
  (params (NewParam :type Boolean))
  (if NewParam
    (`MaterialInstanceDynamic.SetScalarParameterValue` (`self.material`) "Emissive" (`self.materialLightOn`))
    (else
      (`MaterialInstanceDynamic.SetScalarParameterValue` (`self.material`) "Emissive" (`self.materialLightOff`)))))

(fn `UserConstructionScript`
  (bind _active (`self.Active`))
  (`SceneComponent.SetVisibility` (`self.PointLight`) _active false)
  (`SceneComponent.SetVisibility` (`self.SpotLight1`) _active false)
  (bind _returnvalue (`PrimitiveComponent.CreateDynamicMaterialInstance` (`self.SM_TableLamp`) 0 "/Game/TeamContent/Graphic/Material/MaterialInstance/MI_PrpsUVset1_2.MI_PrpsUVset1_2" "None"))
  (set `self.material` _returnvalue)
  (`self.LightOn/Off` _active))