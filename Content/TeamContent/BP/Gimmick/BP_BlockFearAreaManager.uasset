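; BP_BlockFearAreaManager is a manager that answers queries about the BP_BlockFearArea gimmick actors in the level.
; On BeginPlay it caches every such area into an Areas array.
; IsInArea reports whether a position lies within the BFAreaRadius of any active area, using a simple distance check.
; GetIsActive returns the active state of an area by its index in that gathered array.
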(event `self.ReceiveBeginPlay`
  (bind _outactors (`GameplayStatics.GetAllActorsOfClass` "/Game/TeamContent/BP/Gimmick/BP_BlockFearArea.BP_BlockFearArea_C"))
  (set `self.Areas` _outactors))

(fn `GetIsActive`
  (params (AreaIndex :type Integer))
  (returns (active :type Boolean))
  (return (`/Game/TeamContent/BP/Gimmick/BP_BlockFearArea.Active` (`|GetArrayItem` (`self.Areas`) AreaIndex))))

(fn `IsInArea`
  (params (origin :type "Vector Structure"))
  (returns (inRange :type Boolean))
  (locals (inArea :type Boolean))
  (for _array_element (`self.Areas`)
    (if (`/Game/TeamContent/BP/Gimmick/BP_BlockFearArea.Active` _array_element)
      (if (< (`KismetMathLibrary.Vector_Distance` (`self.K2_GetActorLocation` _array_element) origin) (`/Game/TeamContent/BP/Gimmick/BP_GimmickData.BF_AreaRadius` (`/Game/TeamContent/BP/Gimmick/BP_GimickBase.GimmickParam` _array_element)))
        (set `local.inArea` true))))
  (return (`local.inArea`)))

(fn `UserConstructionScript`)