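; BP_RosaryMaker is an interactive gimmick where a player clears timed key-press rounds to earn a rosary effect.
; The server randomizes key and target time each round, checks input against a buffer window, and multicasts updates to the meter widget.
; A miss restarts from round zero, and leaving the box ends play.
; Clearing all rounds messages the player, hides the padlock, and swings the doors open via timeline before play ends.
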(event `self.ReceiveBeginPlay`
  (`SceneComponent.SetVisibility` (`self.Widget`) true false)
  (bind _aswbp_rosary_maker (cast `/Game/TeamContent/BP/UI/WBP_RosaryMaker` (`WidgetComponent.GetWidget` (`self.Widget`))))
  (set `self.MeterWidget` _aswbp_rosary_maker)
  (`KismetSystemLibrary.Delay` 0.1)
  (`SceneComponent.SetVisibility` (`self.Widget`) false false))

(event `self.ReceiveTick`
  (params (DeltaSeconds :type "Float (single-precision)"))
  (`|ExecutionSequence`
    (:`then_0`
      (`self.E_UpdatePlay`))))

(event `RoS_SetSelectKey`
  ;[1 1 1] ランダムキーを設定
  (`self.MC_SetSelectKey` (`/Game/TeamContent/BP/FunctionLibrary/BPL_RosaryKey.GetRosaryKeyFromIndex` (`KismetMathLibrary.RandomIntegerInRange` 0 7))))

(event `MC_SetSelectKey`
  (params (SelectKey :type "Key Structure" :default "None"))
  ;[1 1 1] ランダムキーを設定
  (set `self.SelectKey` SelectKey))

(event `/Game/TeamContent/BP/Gimmick/BPI_GimmickInteface.PlayStart`
  (params (PlayHuman :type "Actor Object Reference"))
  (`self.E_PlayStart` PlayHuman))

(event `/Game/TeamContent/BP/Gimmick/BPI_GimmickInteface.PlayEnd`
  (`self.E_PlayEnd`))

(event `MC_SetIsPlaying`
  (params (isPlaing :type Boolean))
  ;[1 1 1] プレイ中フラグを設定
  (set `self.isPlaing` isPlaing))

(event `E_PlayStart`
  (params (PlayerHuman :type "Actor Object Reference"))
  ;[1 1 1] チャレンジ初回開始
  (`/Engine/EditorBlueprintResources/ActorMacros.Switch Has Authority`
    (:`Authority`
      (if (not (`self.IsGiving`))
        (set `self.PlayerHuman` PlayerHuman)
        (`self.E_SetMaxTimeAndTargetTime`)
        (`self.RoS_SetMeterVisibility` true)
        (`self.MC_SetExplainUIVisibility` false)
        (`self.E_UpdateRound` 0)
        (`self.E_SetState` "NewEnumerator0")
        (`self.MC_SetIsPlaying` true)))))

(event `RoS_SetMeterVisibility`
  (params (bNewVisibility :type Boolean))
  ;[1 1 1] メーターのビジビリティを設定
  (`self.MC_SEtMeterVisibility` bNewVisibility))

(event `MC_SetMeterVisibility`
  (params (bNewVisibility :type Boolean))
  ;[1 1 1] メーターのビジビリティを設定
  (`SceneComponent.SetVisibility` (`self.Widget`) bNewVisibility false))

(event `E_PlayEnd`
  ;[1 1 1] チャレンジ終了
  (`/Engine/EditorBlueprintResources/ActorMacros.Switch Has Authority`
    (:`Authority`
      (if (not (`self.IsGiving`))
        (message `/Game/TeamContent/BP/Player/InGame/Human/BPI_HumanInterface.RosaryPlayEnd` (`self.PlayerHuman`))
        (set `self.PlayerHuman` null)
        (`self.E_UpdateRound` 0)
        (`self.RoS_SetMeterVisibility` false)
        (`self.MC_SetExplainUIVisibility` true)
        (`self.MC_SetPadLocVisibility` true)
        (`self.MC_SetIsPlaying` false)))))

(event `MC_SetExplainUIVisibility`
  (params (bNewVisibility :type Boolean))
  ;[1 1 1] 説明UIのVisibility設定
  (`SceneComponent.SetVisibility` (`self.Widget1`) bNewVisibility false))

(event `E_UpdatePlay`
  ;[1 1 1] タイマー更新
  (`/Engine/EditorBlueprintResources/ActorMacros.Switch Has Authority`
    (:`Authority`
      (if (and (`self.isPlaing`) (`|EnumEquality` (`self.State`) "NewEnumerator0"))
        (set `self.CurrentTime` (+ (`self.CurrentTime`) (`GameplayStatics.GetWorldDeltaSeconds`)))
        (`self.MC_UpdateMeterUI` (`self.CurrentTime`))
        (if (>= (`self.CurrentTime`) (+ (`self.TargetTime`) (* (`/Game/TeamContent/BP/Gimmick/BP_RosaryData.InputBuffer` (`self.Data`)) 0.5)))
          (`self.E_Fail`))))))

(event `MC_UpdateMeterUI`
  (params (CurrentTime :type "Float (double-precision)"))
  ;[1 1 1] メーターUIをMC更新
  (bind _meterwidget (`self.MeterWidget`)
    (:`then`
      (`/Game/TeamContent/BP/UI/WBP_RosaryMaker.E_UpdateCurrentTIme` _meterwidget CurrentTime))
    (:`else`)))

(event `E_SetMaxTimeAndTargetTime`
  (bind _data (`self.Data`))
  ;[1 1 1] 全体時間と目標時間を設定
  (`/Engine/EditorBlueprintResources/ActorMacros.Switch Has Authority`
    (:`Authority`
      (bind _output_get (set `self.MaxTime` (`KismetMathLibrary.RandomFloatInRange` (`/Game/TeamContent/BP/Gimmick/BP_RosaryData.MaxTime_Min` _data) (`/Game/TeamContent/BP/Gimmick/BP_RosaryData.MaxTime_Max` _data))))
      (set `self.CurrentTime` 0.0)
      (bind _returnvalue (* _output_get 0.2))
      (set `self.TargetTime` (`KismetMathLibrary.RandomFloatInRange` _returnvalue (- (`self.MaxTime`) _returnvalue)))
      (`self.RoS_SetSelectKey`)
      (`self.MC_InitMeterUI` (`self.MaxTime`) (`self.TargetTime`)))))

(event `MC_InitMeterUI`
  (params (MaxTime :type "Float (double-precision)") (TargetTime :type "Float (double-precision)"))
  ;[1 1 1] メーターUIをMC初期化
  (bind _meterwidget (`self.MeterWidget`)
    (:`then`
      (`/Game/TeamContent/BP/UI/WBP_RosaryMaker.E_InitMeter` _meterwidget MaxTime TargetTime (`/Game/TeamContent/BP/Gimmick/BP_RosaryData.InputBuffer` (`self.Data`)) (`self.SelectKey`)))
    (:`else`)))

(event `E_Fail`
  ;[1 1 1] 失敗
  (`self.E_PlayStart` (`self.PlayerHuman`)))

(event `E_Success`
  ;[1 1 1] 入力成功
  (`self.E_SetMaxTimeAndTargetTime`)
  (`self.E_SetState` "NewEnumerator0"))

(event `/Game/TeamContent/BP/Gimmick/BPI_GimmickInteface.TryInput`
  (params (NewParam :type "Key Structure"))
  (bind _returnvalue (* (`/Game/TeamContent/BP/Gimmick/BP_RosaryData.InputBuffer` (`self.Data`)) 0.5))
  ;[1 1 1] 入力
  (`/Engine/EditorBlueprintResources/ActorMacros.Switch Has Authority`
    (:`Authority`
      (if (not (`self.IsGiving`))
        (if (== (`self.SelectKey`) NewParam)
          (if (and (>= (`self.CurrentTime`) (- (`self.TargetTime`) _returnvalue)) (<= (`self.CurrentTime`) (+ _returnvalue (`self.TargetTime`))))
            (`self.E_UpdateRound` (+ (`self.CurrentChallengeNum`) 1))
            (if (== (`self.CurrentChallengeNum`) (`/Game/TeamContent/BP/Gimmick/BP_RosaryData.MaxChallengeNum` (`self.Data`)))
              (`self.E_SetState` "NewEnumerator1")
              (`self.E_AllSuccess`)
              (else
                (`self.E_SetState` "NewEnumerator1")
                (`KismetSystemLibrary.Delay` (`/Game/TeamContent/BP/Gimmick/BP_RosaryData.SuccessInterval` (`self.Data`)))
                (`self.E_Success`)))
            (else
              (`self.E_SetState` "NewEnumerator1")
              (`KismetSystemLibrary.Delay` (`/Game/TeamContent/BP/Gimmick/BP_RosaryData.SuccessInterval` (`self.Data`)))
              (if (`self.isPlaing`)
                (`self.E_Fail` :!label _label))))
          (else
            (goto _label)))))))

(event `MC_SetRoundUI`
  (params (CurrentRound :type Integer))
  ;[1 1 1] ラウンドを設定
  (bind _meterwidget (`self.MeterWidget`)
    (:`then`
      (`/Game/TeamContent/BP/UI/WBP_RosaryMaker.E_SetRound` _meterwidget CurrentRound (`/Game/TeamContent/BP/Gimmick/BP_RosaryData.MaxChallengeNum` (`self.Data`))))
    (:`else`)))

(event `E_UpdateRound`
  (params (Round :type Integer))
  ;[1 1 1] ラウンドを設定
  (set `self.CurrentChallengeNum` (`KismetMathLibrary.Clamp` Round 0 (`/Game/TeamContent/BP/Gimmick/BP_RosaryData.MaxChallengeNum` (`self.Data`))))
  (`self.MC_SetRoundUI` (`self.CurrentChallengeNum`)))

(event `E_AllSuccess`
  ;[1 1 1] 全ラウンド成功
  (set `self.IsGiving` true)
  (message `/Game/TeamContent/BP/Player/InGame/Human/BPI_HumanInterface.GetRosary` (`self.PlayerHuman`) (`/Game/TeamContent/BP/Gimmick/BP_RosaryData.EffectRange` (`self.Data`)) (`/Game/TeamContent/BP/Gimmick/BP_RosaryData.EffectTime` (`self.Data`)))
  (`self.MC_SetPadLocVisibility` false)
  (`KismetSystemLibrary.Delay` 0.3)
  (`self.RoS_SetMeterVisibility` false)
  (`self.E_OpenClose`))

(event `E_SetState`
  (params (State :type "/Game/TeamContent/BP/Enum/En_RosaryMakerState Enum" :default "NewEnumerator0"))
  ;[1 1 1] ステートを設定
  (set `self.State` State))

(event `self.Box.OnComponentEndOverlap`
  (params (OverlappedComponent :type "PrimitiveComponent Object Reference") (OtherActor :type "Actor Object Reference") (OtherComp :type "PrimitiveComponent Object Reference") (OtherBodyIndex :type Integer))
  (if (== OtherActor (`self.PlayerHuman`))
    (`self.E_PlayEnd`)))

(event `MC_SetDoorRotation`
  (params (rightDoorRot :type "Rotator Structure") (LeftDoorRot :type "Rotator Structure"))
  ;[1 1 1] ドアオープン
  (`SceneComponent.K2_SetRelativeRotation` (`self.RightDoor`) rightDoorRot false false)
  (`SceneComponent.K2_SetRelativeRotation` (`self.LeftDoor`) LeftDoorRot false false))

(event `E_OpenClose`
  ;[1 1 1] ドアオープン
  (bind (_direction `_新規track_0`) (`Timeline|タイムライン_0` :!via `PlayFromStart`)
    (:`Update`
      (bind _returnvalue (`KismetMathLibrary.Lerp` 0.0 -90.0 `_新規track_0`))
      (`self.MC_SetDoorRotation` (`KismetMathLibrary.MakeRotator` 0.0 0.0 _returnvalue) (`KismetMathLibrary.MakeRotator` 0.0 0.0 (* _returnvalue -1.0))))
    (:`Finished`
      (set `self.IsGiving` false)
      (`self.E_PlayEnd`))))

(event `MC_SetPadLocVisibility`
  (params (bNewVisibility :type Boolean))
  ;[1 1 1] 南京錠の可視性を設定
  (`SceneComponent.SetVisibility` (`self.PadLoc`) bNewVisibility false))

(fn `F_GetRosarySpawnTransform`
  (returns (transform :type "Transform Structure"))
  (return (`KismetMathLibrary.MakeTransform` (`KismetMathLibrary.MakeVector` (.x (+ (`self.K2_GetActorLocation`) (* (`self.GetActorForwardVector`) 200.0))) (.y (+ (`self.K2_GetActorLocation`) (* (`self.GetActorForwardVector`) 200.0))) 66.0) (`self.K2_GetActorRotation`))))

(fn `IsCanPlay`
  (params (Player :type "Actor Object Reference"))
  (returns (playing :type Boolean))
  (return (and (not (`self.isPlaing`)) (`PrimitiveComponent.IsOverlappingActor` (`self.Box`) Player))))

(fn `UserConstructionScript`)