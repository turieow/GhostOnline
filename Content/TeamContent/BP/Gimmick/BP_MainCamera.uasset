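; BP_MainCamera is a fixed-origin camera actor with a timed zoom to a location and a mode that tracks a target actor.
; E_Zoom, ignored while targeting or already zooming, uses timelines to move the camera in front of the location and back after a delay.
; While targeting, Tick smoothly turns toward the actor and shifts height by its distance change; otherwise it restores the origin.
; Field of view steps toward the requested value, or the default when untargeted.
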(event `self.ReceiveBeginPlay`
  (set `self.OriginTransform` (`SceneComponent.K2_GetComponentToWorld` (`self.SceneComponent`))))

(event `self.ReceiveTick`
  (params (DeltaSeconds :type "Float (single-precision)"))
  (bind _origintransform (`self.OriginTransform`))
  (bind _location (.location (`self.OriginTransform`)))
  (`self.IsTarget`)
  (`self.SetFieldOfView`)
  (`CameraComponent.SetFieldOfView` (`self.CameraComponent`) (`self.NowFieldOfView`))
  (if (not (`self.IsTargetState`))
    (if (not (== _origintransform (`SceneComponent.K2_GetComponentToWorld` (`self.SceneComponent`))))
      (`SceneComponent.K2_SetWorldTransform` (`self.SceneComponent`) _origintransform false false))
    (else
      (`SceneComponent.K2_SetWorldLocation` (`self.SceneComponent`) (`KismetMathLibrary.MakeVector` (.x _location) (.y _location) (- (.z _location) (* (- (`self.targetLength`) (`KismetMathLibrary.VSize` (- _location (`self.K2_GetActorLocation` (`self.TargetActor`))))) 0.8))) false false))))

(event `E_Zoom`
  (params (Location :type "Vector Structure") (Duration :type "Float (double-precision)"))
  (if (not (`self.IsTargetState`))
    (`/Engine/EditorBlueprintResources/StandardMacros.DoOnce` false :!label _label
      (:`Completed`
        (if (not (`self.Zooming`))
          (set `self.Zooming` true)
          (set `self.TargetLoc` (`self.GetTargetTransform` Location (`self.Length`)))
          (bind (_direction _alpha) (`Timeline|ZoomIn` :!via `PlayFromStart`)
            (:`Update`
              (`SceneComponent.K2_SetWorldTransform` (`self.CameraComponent`) (`KismetMathLibrary.TLerp` (`self.OriginTransform`) (`self.TargetLoc`) _alpha) false false))
            (:`Finished`
              (`KismetSystemLibrary.Delay` Duration)
              (bind (_direction_2 _alpha_2) (`Timeline|タイムライン_0` :!via `PlayFromStart`)
                (:`Update`
                  (`SceneComponent.K2_SetWorldTransform` (`self.CameraComponent`) (`KismetMathLibrary.TLerp` (`self.TargetLoc`) (`self.OriginTransform`) _alpha_2) false false))
                (:`Finished`
                  (set `self.Zooming` false)
                  (goto _label :!via `Reset`))))))))))

(event `E_TargetCamera`
  (params (NewParam :type "Actor Object Reference") (NewParam2 :type "Float (double-precision)"))
  (`/Engine/EditorBlueprintResources/StandardMacros.IsValid` NewParam
    (:`Is Valid`
      (set `self.TargetActor` NewParam)
      (set `self.targetLength` (`KismetMathLibrary.VSize` (- (.location (`self.OriginTransform`)) (`self.K2_GetActorLocation` NewParam))))
      (set `self.FieldOfView` NewParam2)
      (set `self.IsTargetState` true))))

(event `E_DisTarget`
  (set `self.IsTargetState` false))

(event `IsTarget`
  (bind _scenecomponent (`self.SceneComponent`))
  (if (`self.IsTargetState`)
    (`SceneComponent.K2_SetWorldRotation` (`self.SceneComponent`) (`KismetMathLibrary.RInterpTo` (`SceneComponent.K2_GetComponentRotation` _scenecomponent) (`KismetMathLibrary.FindLookAtRotation` (`SceneComponent.K2_GetComponentLocation` _scenecomponent) (`self.K2_GetActorLocation` (`self.TargetActor`))) (`GameplayStatics.GetWorldDeltaSeconds`) 7.0) false false)
    (else
      (set `self.FieldOfView` 90.0))))

(event `SetFieldOfView`
  (bind _returnvalue (* 50.0 (`GameplayStatics.GetWorldDeltaSeconds`)))
  (if (< (`KismetMathLibrary.Abs` (- (`self.NowFieldOfView`) (`self.FieldOfView`))) 1.0)
    (set `self.NowFieldOfView` (`self.FieldOfView`))
    (elif (> (- (`self.NowFieldOfView`) (`self.FieldOfView`)) 0.0)
      (set `self.NowFieldOfView` (- (`self.NowFieldOfView`) _returnvalue))
      (else
        (set `self.NowFieldOfView` (+ (`self.NowFieldOfView`) _returnvalue))))))

(fn `GetTargetTransform`
  (params (InVec :type "Vector Structure") (Length :type "Float (double-precision)" :default 500.0))
  (returns (ReturnValue :type "Transform Structure"))
  (bind (_origintransform_location _origintransform_rotation) (`KismetMathLibrary.BreakTransform` (`self.OriginTransform`)))
  (return (`KismetMathLibrary.MakeTransform` (+ InVec (* (* (`SceneComponent.GetForwardVector` (`self.CameraComponent`)) -1.0) Length)) _origintransform_rotation)))

(fn `UserConstructionScript`)