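; Game mode for a multi-round humans-versus-ghost party game, where the current game number picks the ghost player.
; Ghost death or all humans dying awards points, then the Result graph adds round scores to GameInstance totals and shows ranked UI and characters.
; It then fades and reloads the level, or after the last round shows final results and opens L_Main.
; It also offers camera and countdown helpers, but BeginPlay and Tick are empty.
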(event `self.ReceiveBeginPlay`)

(event `self.ReceiveTick`
  (params (DeltaSeconds :type "Float (single-precision)")))

(event `self.ChangeScene`
  (params (NowLevel :type Name) (NextLevel :type Name))
  (bind _returnvalue (`GameplayStatics.GetPlayerCameraManager` 0))
  (if (not (== NowLevel NextLevel))
    (`PlayerCameraManager.StartCameraFade` :`self` _returnvalue :`ToAlpha` 1.0 :`Duration` 0.5)
    (`KismetSystemLibrary.Delay` 0.4)
    (`GameplayStatics.LoadStreamLevel` NextLevel)
    (`GameplayStatics.UnloadStreamLevel` NowLevel)
    (`GameplayStatics.OpenLevel` NextLevel)
    (else
      (`PlayerCameraManager.StartCameraFade` :`self` _returnvalue :`ToAlpha` 1.0 :`Duration` 0.5)
      (`KismetSystemLibrary.Delay` 0.4)
      (`GameplayStatics.UnloadStreamLevel` NowLevel)
      (`GameplayStatics.OpenLevel` NextLevel))))

(event `E_CreateMainUI`
  ;[1 1 1] MainUIを作成
  (bind _returnvalue (`|CreateWidget` "/Game/TeamContent/BP/UI/WBP_Main.WBP_Main_C"))
  (bind _output_get (set `self.MainUI` _returnvalue))
  (`UserWidget.AddToViewport` _output_get 0))

(event `self.ZoomCamera`
  (params (CharacterLoc :type "Vector Structure") (Duraction :type "Float (single-precision)"))
  (bind _cameraactor (`self.CameraActor`)
    (:`then`
      (`/Game/TeamContent/BP/Gimmick/BP_MainCamera.E_Zoom` _cameraactor CharacterLoc Duraction))
    (:`else`)))

(event `E_GetCreatePlayerManager`
  ;[1 1 1] レベルのアクタ取得
  (bind _outactors (`GameplayStatics.GetAllActorsOfClass` "/Game/TeamContent/BP/Player/InGame/Manager/BP_PlayerSpawnManager.BP_PlayerSpawnManager_C"))
  (if (`KismetArrayLibrary.Array_IsValidIndex` _outactors)
    (set `self.CreatePlayerManager` (`|GetArrayItem` _outactors))
    (else
      (bind _returnvalue (`|SpawnActorFromClass` "/Game/TeamContent/BP/Player/InGame/Manager/BP_PlayerSpawnManager.BP_PlayerSpawnManager_C" (`KismetMathLibrary.MakeTransform` (0.0 0.0 0.0)) "Undefined" "OverrideRootScale" null 1 null))
      (set `self.CreatePlayerManager` _returnvalue))))

(event `E_GetCameraActor`
  ;[1 1 1] レベルのアクタ取得
  (bind _outactors (`GameplayStatics.GetAllActorsOfClass` "/Game/TeamContent/BP/Gimmick/BP_MainCamera.BP_MainCamera_C"))
  (if (`KismetArrayLibrary.Array_IsValidIndex` _outactors)
    (set `self.CameraActor` (`|GetArrayItem` _outactors))))

(event `self.FinishGame`
  (`self.E_InitResult`))

(event `self.GhostDead`
  ;[1 1 1] お化け死亡
  (set `self.State` "NewEnumerator2")
  (`|ExecutionSequence`
    (:`then_0`
      (bind _currentgamenum (message `/Game/TeamContent/BP/System/GameInstance/BPI_GameInstanceInterface.GetCurrentGameNum` (`GameplayStatics.GetGameInstance`)))
      (bind _playercontroller (message `/Game/TeamContent/BP/System/GameInstance/BPI_GameInstanceInterface.GetMyPlayerController` (`GameplayStatics.GetGameInstance`) _currentgamenum))
      (bind _returnvalue (`self.GetNumPlayers` (`GameplayStatics.GetGameMode`)))
      (for _index (range _returnvalue)
        (bind _playercontroller_2 (message `/Game/TeamContent/BP/System/GameInstance/BPI_GameInstanceInterface.GetMyPlayerController` (`GameplayStatics.GetGameInstance`) _index))
        (if (!= _playercontroller_2 _playercontroller)
          (bind _returnvalue_2 (`Controller.K2_GetPawn` _playercontroller_2))
          (message `/Game/TeamContent/BP/Player/InGame/Player/BPI_Player.AddScore` _returnvalue_2 2)
          (bind _isalive (message `/Game/TeamContent/BP/Player/InGame/Human/BPI_HumanInterface.GetIsAlive` _returnvalue_2))
          (if _isalive
            (message `/Game/TeamContent/BP/Player/InGame/Player/BPI_Player.AddScore` _returnvalue_2 1) ; 生き残ってた人に１PT
          ))))
    (:`then_2`
      (`self.E_InitResult`))))

(event `self.AllHumanDead`
  ;[1 1 1] 全人類死亡
  (set `self.State` "NewEnumerator1")
  (`|ExecutionSequence`
    (:`then_0`
      (bind _currentgamenum (message `/Game/TeamContent/BP/System/GameInstance/BPI_GameInstanceInterface.GetCurrentGameNum` (`GameplayStatics.GetGameInstance`)))
      (bind _playercontroller (message `/Game/TeamContent/BP/System/GameInstance/BPI_GameInstanceInterface.GetMyPlayerController` (`GameplayStatics.GetGameInstance`) _currentgamenum))
      (bind _returnvalue (`self.GetNumPlayers` (`GameplayStatics.GetGameMode`)))
      (for _index (range _returnvalue)
        (bind _playercontroller_2 (message `/Game/TeamContent/BP/System/GameInstance/BPI_GameInstanceInterface.GetMyPlayerController` (`GameplayStatics.GetGameInstance`) _index))
        (if (!= _playercontroller_2 _playercontroller)
          (bind _returnvalue_2 (`Controller.K2_GetPawn` _playercontroller_2))
          (message `/Game/TeamContent/BP/Player/InGame/Human/BPI_HumanInterface.CommitOnDeadPoint` _returnvalue_2)
          (else
            (bind _newparam (message `/Game/TeamContent/BP/Player/InGame/Ghost/BPI_GhostInterface.GetGhostManager` _returnvalue_2))
            (message `/Game/TeamContent/BP/Player/InGame/Ghost/BPI_GhostInterface.AddGhostScore` _newparam 2)))))
    (:`then_1`
      (`self.E_InitResult`))))

(event `self.HumanDead`
  (bind _result (`/Engine/EditorBlueprintResources/StandardMacros.IncrementInt` (`self.DeadHumanNum`))
    (:`  `
      (if (== _result (`self.MaxHumanNum`))
        (`KismetSystemLibrary.Delay` 2.0)
        (`self.AllHumanDead`)))))

(event `ResetTime`
  ;[1 1 1] CountDown系
  (set `self.NowTime` (`self.TimeLimit`)))

(event `CountDownTime`
  ;[1 1 1] CountDown系
  (if (`self.IsCountDown`)
    (bind _output_get (set `self.NowTime` (- (`self.NowTime`) (`GameplayStatics.GetWorldDeltaSeconds`))))
    (if (<= _output_get 0.0)
      (set `self.IsTimeUp` true)
      (set `self.NowTime` 0.0)
      (else
        (set `self.IsTimeUp` false)))))

(event `self.SetCountDownFlag`
  (params (flag :type Boolean))
  ;[1 1 1] CountDown系
  (set `self.IsCountDown` flag))

(event `TimeUp`
  (if (`self.IsTimeUp`)
    (`/Engine/EditorBlueprintResources/StandardMacros.DoOnce` false :!label _label)
    (else
      (goto _label :!via `Reset`))))

(event `Key|AnyKey`
  (params (Key :type "Key Structure"))
  (:`Pressed`
    (`KismetSystemLibrary.PrintString` (`KismetStringLibrary.Conv_NameToString` (`.MotionSource` (`HeadMountedDisplayFunctionLibrary.BreakKey` Key))))))

(event `self.Debug_TimeUp`
  (set `self.NowTime` 1.0))

(event `self.StartTargetCamera`
  (params (target :type "Actor Object Reference") (CameraVolumu :type "Float (single-precision)"))
  (bind _cameraactor (`self.CameraActor`)
    (:`then`
      (`/Game/TeamContent/BP/Gimmick/BP_MainCamera.E_TargetCamera` _cameraactor target CameraVolumu))
    (:`else`)))

(event `self.DisTargetCamera`
  (bind _cameraactor (`self.CameraActor`)
    (:`then`
      (`/Game/TeamContent/BP/Gimmick/BP_MainCamera.E_DisTarget` _cameraactor))
    (:`else`)))

(event `E_InitResult`
  (bind _mainui (`self.MainUI`)
    (:`then`
      (message `/Game/TeamContent/BP/UI/BPI_ToUI.FadeOut` _mainui 1.0)
      (`KismetSystemLibrary.Delay` 1.0)
      (bind _resultdata (`self.CreateResultData`))
      (bind _output_get (set `self.Result Data` _resultdata))
      (`self.E_CreateResultUI` _output_get)
      (`self.E_CreateResultCharacter` false)
      (bind _outactors (`GameplayStatics.GetAllActorsWithTag` "ResultCamera"))
      (if (`KismetArrayLibrary.Array_IsValidIndex` _outactors)
        (`PlayerController.SetViewTargetWithBlend` (`GameplayStatics.GetPlayerController` 0) (`|GetArrayItem` _outactors) 0.0 "VTBlend_Linear" 0.0 false)
        ;[1 0.8273 0] TODO:CurrentGameNumを確認して次のゲームへ進む処理
        (message `/Game/TeamContent/BP/System/GameInstance/BPI_GameInstanceInterface.AddCurrentGameNum` (`GameplayStatics.GetGameInstance`))
        (bind _gamenum (message `/Game/TeamContent/BP/System/GameInstance/BPI_GameInstanceInterface.IsMaxGameNum?` (`GameplayStatics.GetGameInstance`)))
        (if _gamenum
          (`KismetSystemLibrary.Delay` 5.0)
          (bind _resultui (`self.ResultUI`)
            (:`then`
              (message `/Game/TeamContent/BP/UI/BPI_ToUI.FadeOut` _resultui 1.0)
              (`KismetSystemLibrary.Delay` 1.0)
              (`self.E_ClearResultCharacters`)
              (`self.E_CreateResultCharacter` true)
              (`Widget.RemoveFromParent` (`self.ResultUI`))
              (`self.E_CreateResultUI` (`self.Result Data`) true)
              (`KismetSystemLibrary.Delay` 5.0)
              (bind _resultui_2 (`self.ResultUI`)
                (:`then`
                  (message `/Game/TeamContent/BP/UI/BPI_ToUI.FadeAnimation` _resultui_2 true 1.0)
                  (`KismetSystemLibrary.Delay` 1.0)
                  (`GameplayStatics.OpenLevelBySoftObjectPtr` "/Game/TeamContent/Level/Online/L_Main.L_Main"))
                (:`else`)))
            (:`else`))
          (else
            (`KismetSystemLibrary.Delay` 5.0)
            (bind _resultui_3 (`self.ResultUI`)
              (:`then`
                (message `/Game/TeamContent/BP/UI/BPI_ToUI.FadeOut` _resultui_3 1.0)
                (`KismetSystemLibrary.Delay` 1.0)
                (bind _returnvalue (`GameplayStatics.GetCurrentLevelName` true))
                (bind _returnvalue_2 (`KismetStringLibrary.Conv_StringToName` _returnvalue))
                (`self.ChangeScene` _returnvalue_2 _returnvalue_2))
              (:`else`))))))
    (:`else`)))

(event `E_CreateResultUI`
  (params (NewParam :type "Array of /Game/TeamContent/BP/Struct/ST_ResultValue Structure (by ref)") (IsFinalResult :type Boolean))
  (bind _returnvalue (`|CreateWidget` "/Game/TeamContent/BP/UI/WBP_Result.WBP_Result_C" null IsFinalResult))
  (bind _output_get (set `self.ResultUI` _returnvalue))
  (`UserWidget.AddToViewport` _output_get 0)
  (`/Game/TeamContent/BP/UI/WBP_Result.E_InitResultUI` _returnvalue NewParam 40)
  (bind _mainui (`self.MainUI`)
    (:`then`
      (`Widget.RemoveFromParent` _mainui))
    (:`else`)))

(event `E_CreateResultCharacter`
  (params (IsFinalResult :type Boolean))
  (bind _controllerindexandjunni1 (`self.GetPlayerJunni` (`self.Result Data`)))
  (bind _values (`BlueprintMapLibrary.Map_Values` _controllerindexandjunni1))
  (for _array_element (`self.Result Data`)
    (bind (_point _controllerindex) (break `/Game/TeamContent/BP/Struct/ST_ResultValue` _array_element))
    (bind _returnvalue (`|SpawnActorFromClass` "/Game/TeamContent/BP/Player/Result/BP_ResultRenderCamera.BP_ResultRenderCamera_C" (`KismetMathLibrary.MakeTransform` (0.0 0.0 0.0)) "Undefined" "OverrideRootScale" null _controllerindex (`|GetArrayItem` _values _controllerindex) IsFinalResult null))
    (`KismetArrayLibrary.Array_Add` (`self.ResultCharacters`) _returnvalue)))

(event `E_ClearResultCharacters`
  ;[1 1 1] リザルトキャラクターを削除
  (for _array_element (`self.ResultCharacters`)
    (`self.K2_DestroyActor` _array_element))
  (`KismetArrayLibrary.Array_Clear` (`self.ResultCharacters`)))

(event `self.K2_PostLogin`
  (params (NewPlayer :type "PlayerController Object Reference"))
  (`KismetArrayLibrary.Array_Add` (`self.ControllersRef`) NewPlayer)
  (bind _asgs_main (cast `/Game/TeamContent/BP/System/MainGame/GS_Main` (`GameplayStatics.GetGameState`)))
  (`/Game/TeamContent/BP/System/MainGame/GS_Main.E_PlayerLogin` _asgs_main NewPlayer))

(fn `CreateResultData`
  (returns (ResultData :type "Array of /Game/TeamContent/BP/Struct/ST_ResultValue Structure"))
  (locals (SortedResultData :type "Array of /Game/TeamContent/BP/Struct/ST_ResultValue Structure") (ControllerIndex :type Integer) (PlayerScore :type Integer))
  (for _index (range 4)
    (bind _playercontroller (message `/Game/TeamContent/BP/System/GameInstance/BPI_GameInstanceInterface.GetMyPlayerController` (`GameplayStatics.GetGameInstance`) _index))
    (set `local.ControllerIndex` (`GameplayStatics.GetPlayerControllerID` _playercontroller))
    (`|ExecutionSequence`
      (:`then_0`
        (bind _currentgamenum (message `/Game/TeamContent/BP/System/GameInstance/BPI_GameInstanceInterface.GetCurrentGameNum` (`GameplayStatics.GetGameInstance`)))
        (bind _playercontroller_2 (message `/Game/TeamContent/BP/System/GameInstance/BPI_GameInstanceInterface.GetMyPlayerController` (`GameplayStatics.GetGameInstance`) _currentgamenum))
        (if (== _playercontroller_2 _playercontroller)
          ;[1 1 1] お化けの場合
          (`/Engine/EditorBlueprintResources/StandardMacros.IsValid` (`GameplayStatics.GetPlayerController` (`local.ControllerIndex`))
            (:`Is Valid`
              (bind _returnvalue (`Controller.K2_GetPawn` _playercontroller_2))
              (`/Engine/EditorBlueprintResources/StandardMacros.IsValid` _returnvalue
                (:`Is Valid`
                  (bind _newparam (message `/Game/TeamContent/BP/Player/InGame/Ghost/BPI_GhostInterface.GetGhostManager` _returnvalue))
                  (`/Engine/EditorBlueprintResources/StandardMacros.IsValid` _newparam
                    (:`Is Valid`
                      (set `local.PlayerScore` (`/Game/TeamContent/BP/Player/InGame/Manager/BP_GhostManager.Score` _newparam)))))
                (:`Is Not Valid`
                  ;;[0.05117 0.9602 1] Debug:ゴーストが設定されていないとき用
                  (bind _outactors (`GameplayStatics.GetAllActorsOfClass` "/Game/TeamContent/BP/Player/InGame/Ghost/BP_Ghost.BP_Ghost_C" :!label _label))
                  (set `local.PlayerScore` (`/Game/TeamContent/BP/Player/InGame/Manager/BP_GhostManager.Score` (`/Game/TeamContent/BP/Player/InGame/Player/BP_Player.Manager` (`|GetArrayItem` _outactors)))))))
            (:`Is Not Valid`
              (goto _label)))
          (else
            ;[1 1 1] 人間の場合
            (bind _point (message `/Game/TeamContent/BP/Player/InGame/Player/BPI_Player.GetScore` (`Controller.K2_GetPawn` (`GameplayStatics.GetPlayerController` (`local.ControllerIndex`)))))
            (set `local.PlayerScore` _point))))
      (:`then_1`
        (bind _point_2 (message `/Game/TeamContent/BP/System/GameInstance/BPI_GameInstanceInterface.GetPlayerPointData` (`GameplayStatics.GetGameInstance`) (`local.ControllerIndex`)))
        (bind _returnvalue_2 (+ _point_2 (`local.PlayerScore`)))
        (`KismetArrayLibrary.Array_Add` (`local.SortedResultData`) (make `/Game/TeamContent/BP/Struct/ST_ResultValue` _returnvalue_2 (`local.ControllerIndex`) _point_2))
        (message `/Game/TeamContent/BP/System/GameInstance/BPI_GameInstanceInterface.SetPlayerPointData` (`GameplayStatics.GetGameInstance`) (`local.ControllerIndex`) _returnvalue_2))))
  (return (`local.SortedResultData`)))

(fn `CreateSortedResultData`
  (returns (ResultData :type "Array of /Game/TeamContent/BP/Struct/ST_ResultValue Structure"))
  (locals (FirstPlayers :type "Array of Actor Object Reference") (FirstPoints :type "Array of Integer") (SortedResultData :type "Array of /Game/TeamContent/BP/Struct/ST_ResultValue Structure") (FirstControllerID :type "Array of Integer"))
  (bind (_indexofmaxvalue _maxvalue) (`KismetMathLibrary.MaxOfIntArray` (`local.FirstPoints`)))
  (bind _output (`|GetArrayItem` (`local.FirstControllerID`) _indexofmaxvalue))
  (bind _createplayermanager (`self.CreatePlayerManager`)
    (:`then`
      (set `local.FirstPlayers` (`/Game/TeamContent/BP/Player/InGame/Manager/BP_PlayerSpawnManager.Humans` _createplayermanager))
      (bind _currentgamenum (message `/Game/TeamContent/BP/System/GameInstance/BPI_GameInstanceInterface.GetCurrentGameNum` (`GameplayStatics.GetGameInstance`)))
      (bind _returnvalue (`GameplayStatics.GetPlayerController` _currentgamenum))
      (`/Engine/EditorBlueprintResources/StandardMacros.IsValid` _returnvalue
        (:`Is Valid`
          (bind _returnvalue_2 (`Controller.K2_GetPawn` _returnvalue))
          (`/Engine/EditorBlueprintResources/StandardMacros.IsValid` _returnvalue_2
            (:`Is Valid`
              (bind _newparam (message `/Game/TeamContent/BP/Player/InGame/Ghost/BPI_GhostInterface.GetGhostManager` _returnvalue_2))
              (`/Engine/EditorBlueprintResources/StandardMacros.IsValid` _newparam
                (:`Is Valid`
                  (bind _playerghost (`/Game/TeamContent/BP/Player/InGame/Manager/BP_GhostManager.PlayerGhost` _newparam))
                  (`/Engine/EditorBlueprintResources/StandardMacros.IsValid` _playerghost
                    (:`Is Valid`
                      (`KismetArrayLibrary.Array_Add` (`local.FirstPlayers`) _playerghost))
                    (:`Is Not Valid`
                      ;[0.05117 0.9602 1] Debug:ゴーストが設定されていないとき用
                      (bind _outactors (`GameplayStatics.GetAllActorsOfClass` "/Game/TeamContent/BP/Player/InGame/Ghost/BP_Ghost.BP_Ghost_C" :!label _label))
                      (bind _output_2 (`|GetArrayItem` _outactors))
                      (set `/Game/TeamContent/BP/Player/InGame/Player/BP_Player.Index` _currentgamenum _output_2)
                      (`KismetArrayLibrary.Array_Add` (`local.FirstPlayers`) _output_2))))
                (:`Is Not Valid`
                  (goto _label))))
            (:`Is Not Valid`
              (goto _label))))
        (:`Is Not Valid`
          (goto _label)))
      (for _array_element (`local.FirstPlayers`)
        (`/Engine/EditorBlueprintResources/StandardMacros.IsValid` _array_element
          (:`Is Valid`
            (bind _id (message `/Game/TeamContent/BP/Player/InGame/Player/BPI_Player.GetControllerID` _array_element))
            (`KismetArrayLibrary.Array_Add` (`local.FirstControllerID`) _id)
            (bind _point (message `/Game/TeamContent/BP/Player/InGame/Player/BPI_Player.GetScore` _array_element))
            (bind _point_2 (message `/Game/TeamContent/BP/System/GameInstance/BPI_GameInstanceInterface.GetPlayerPointData` (`GameplayStatics.GetGameInstance`) _id))
            (`KismetArrayLibrary.Array_Add` (`local.FirstPoints`) (+ _point_2 _point)))))
      (for _ (range (+ (`KismetArrayLibrary.Array_LastIndex` (`local.FirstPlayers`)) 1))
        (bind _point_3 (message `/Game/TeamContent/BP/System/GameInstance/BPI_GameInstanceInterface.GetPlayerPointData` (`GameplayStatics.GetGameInstance`) _output))
        (bind _playercontroller (message `/Game/TeamContent/BP/System/GameInstance/BPI_GameInstanceInterface.GetMyPlayerController` (`GameplayStatics.GetGameInstance`) _output))
        (`KismetArrayLibrary.Array_Add` (`local.SortedResultData`) (make `/Game/TeamContent/BP/Struct/ST_ResultValue` _maxvalue (`GameplayStatics.GetPlayerControllerID` _playercontroller) _point_3))
        (message `/Game/TeamContent/BP/System/GameInstance/BPI_GameInstanceInterface.SetPlayerPointData` (`GameplayStatics.GetGameInstance`) _output _maxvalue)
        (`KismetArrayLibrary.Array_Remove` (`local.FirstControllerID`) _indexofmaxvalue)
        (`KismetArrayLibrary.Array_Remove` (`local.FirstPoints`) _indexofmaxvalue))
      (return (`local.SortedResultData`)))
    (:`else`)))

(fn `GetAngle`
  (params (targetLoc :type "Vector Structure") (OringinLoc :type "Vector Structure") (StanderdLoc :type "Vector Structure") (StanderdVec :type "Vector Structure"))
  (returns (Angle :type "Float (double-precision)"))
  (bind _angle (`self.GetAngleFunction` targetLoc OringinLoc StanderdLoc StanderdVec))
  (return _angle))

(fn `GetAngleFunction`
  (params (TargetLoc :type "Vector Structure") (OriginLoc :type "Vector Structure") (StanderdLoc :type "Vector Structure") (StanderdVec :type "Vector Structure"))
  (returns (Angle :type "Float (double-precision)"))
  (locals (AngleOutPut :type "Float (double-precision)"))
  (bind _returnvalue (`KismetMathLibrary.Normal` (- OriginLoc StanderdLoc) 0.1))
  (bind _returnvalue_2 (`KismetMathLibrary.Normal` (- TargetLoc OriginLoc) 0.1))
  (bind _returnvalue_3 (`KismetMathLibrary.DegAcos` (`KismetMathLibrary.Dot_VectorVector` _returnvalue_2 _returnvalue)))
  (if (< (`KismetMathLibrary.Dot_VectorVector` (`KismetMathLibrary.Cross_VectorVector` _returnvalue_2 _returnvalue) StanderdVec) 0.0)
    (set `local.AngleOutPut` (* _returnvalue_3 1.0))
    (return (`local.AngleOutPut`))
    (else
      (set `local.AngleOutPut` (* _returnvalue_3 -1.0)))))

(fn `GetChangeGhost`
  (params (NewParam :type "Key Structure"))
  (returns (NewParam1 :type "/Game/TeamContent/BP/Player/InGame/Ghost/BP_Ghost Object Reference"))
  (return null))

(fn `GetCountDownFlag`
  (returns (value :type Boolean))
  (return (`self.IsCountDown`)))

(fn `GetDeadHumanNum`
  (returns (deadHumanNum :type Integer))
  (return (`self.DeadHumanNum`)))

(fn `GetGameState`
  (returns (state :type "/Game/TeamContent/BP/Enum/En_GameState Enum"))
  (return (`self.State`)))

(fn `GetHumanActors`
  (returns (humans :type "Array of Actor Object Reference"))
  (bind _createplayermanager (`self.CreatePlayerManager`))
  (`/Engine/EditorBlueprintResources/StandardMacros.IsValid` _createplayermanager
    (:`Is Valid`
      (return (`/Game/TeamContent/BP/Player/InGame/Manager/BP_PlayerSpawnManager.Humans` _createplayermanager)))))

(fn `GetNowCountDownTime`
  (returns (value :type "Float (double-precision)"))
  (return (`self.NowTime`)))

(fn `GetPlayerJunni`
  (params (NewParam :type "Array of /Game/TeamContent/BP/Struct/ST_ResultValue Structure"))
  (returns (ControllerIndexAndJunni1 :type "Map of Integer to Integer"))
  (locals (Points :type "Array of Integer") (ControllerIndexAndJunni :type "Map of Integer to Object Object Reference") (ControllerIDs :type "Array of Integer") (BeforePoint :type Integer) (SameNum :type Integer) (Junni :type Integer :default 0) (JunniLoopNum :type Integer :default 0) (MyPoint :type Integer) (MyControllerIndex :type Integer) (NumOfBiggerScoreThanMine :type Integer))
  (for _index (range 4)
    (set `local.MyControllerIndex` _index)
    (bind _output_point (break `/Game/TeamContent/BP/Struct/ST_ResultValue` (`|GetArrayItem` NewParam _index)))
    (set `local.MyPoint` _output_point)
    (for (_array_element _array_index) NewParam
      (if (!= _array_index (`local.MyControllerIndex`))
        (if (> (`.Point_12_DA4451C84BB85B6D7B2A1FA9D71705A8` (break `/Game/TeamContent/BP/Struct/ST_ResultValue` _array_element)) (`local.MyPoint`))
          (`/Engine/EditorBlueprintResources/StandardMacros.IncrementInt` (`local.NumOfBiggerScoreThanMine`)))))
    (`BlueprintMapLibrary.Map_Add` (`local.ControllerIndexAndJunni`) (`local.MyControllerIndex`) (`local.NumOfBiggerScoreThanMine`))
    (set `local.NumOfBiggerScoreThanMine` 0))
  (return (`local.ControllerIndexAndJunni`)))

(fn `GetResultSpawnLoc`
  (params (BoundsHalf :type "Vector Structure") (CameraLoc :type "Vector Structure"))
  (returns (Location :type "Array of Vector Structure"))
  (locals (Yokohaba :type "Float (double-precision)" :default 0.0) (BottonLeft :type "Vector Structure") (CameraLocation :type "Vector Structure") (Locations :type "Array of Vector Structure"))
  (set `local.CameraLocation` CameraLoc)
  (set `local.Yokohaba` (/ (* 2 (`KismetMathLibrary.Abs` (.y BoundsHalf))) 3.0))
  (set `local.BottonLeft` (+ (`local.CameraLocation`) BoundsHalf))
  (for _index (range 4)
    (`KismetArrayLibrary.Array_Add` (`local.Locations`) (+ (`local.BottonLeft`) (* (`KismetMathLibrary.MakeVector` 0.0 (`local.Yokohaba`)) _index))))
  (return (`local.Locations`)))

(fn `GetTimeUpFlag`
  (returns (value :type Boolean))
  (return (`self.IsTimeUp`)))

(fn `IGetControllersRef`
  (returns (NewParam :type "Array of PlayerController Object Reference"))
  (return (`self.ControllersRef`)))

(fn `UserConstructionScript`)